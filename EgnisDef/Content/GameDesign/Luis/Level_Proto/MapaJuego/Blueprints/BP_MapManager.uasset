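; Map manager that drives node progression on a branching game map, with node states persisted in BP_GI_MapZ1.
; On BeginPlay, after a short delay, it registers every BP_MapNode_Base by ID, unlocks successors of apparently completed nodes, then refreshes visuals.
; SelectNode checks accessibility, saves the choice as current, locks other available nodes and asks the chosen node to enter.
; Locked-out alternatives are saved in a separate state but displayed with the initial state's visual.
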(event `self.ReceiveBeginPlay`
  (bind _gameinstanceref (`self.GameInstanceRef`))
  (bind _asbp_gi_map_z1 (cast `/Game/GameDesign/Luis/Level_Proto/MapaJuego/Blueprints/BP_GI_MapZ1` (`GameplayStatics.GetGameInstance`)))
  (set `self.GameInstanceRef` _asbp_gi_map_z1)
  (bind _outactors (`GameplayStatics.GetAllActorsOfClass` "/Game/GameDesign/Luis/Level_Proto/MapaJuego/Blueprints/BP_MapNode_Base.BP_MapNode_Base_C"))
  (`KismetSystemLibrary.Delay` 0.2)
  (for _array_element _outactors
    (bind _asbp_map_node_base (cast `/Game/GameDesign/Luis/Level_Proto/MapaJuego/Blueprints/BP_MapNode_Base` _array_element))
    (bind _nodeid (`/Game/GameDesign/Luis/Level_Proto/MapaJuego/Blueprints/BP_MapNode_Base.NodeID` _asbp_map_node_base))
    (`self.RegisterNode` _nodeid _asbp_map_node_base)
    (bind _returnvalue (`/Game/GameDesign/Luis/Level_Proto/MapaJuego/Blueprints/BP_GI_MapZ1.GetNodeState` _gameinstanceref _nodeid))
    (if (`|EnumEquality` _returnvalue "NewEnumerator3")
      (`self.UnlockNextNodes` _asbp_map_node_base)))
  (bind _values (`BlueprintMapLibrary.Map_Values` (`self.RegsiteredNodes`)))
  (for _array_element_2 _values
    (bind _nodeid_2 (`/Game/GameDesign/Luis/Level_Proto/MapaJuego/Blueprints/BP_MapNode_Base.NodeID` _array_element_2))
    (bind _returnvalue_2 (`/Game/GameDesign/Luis/Level_Proto/MapaJuego/Blueprints/BP_GI_MapZ1.GetNodeState` _gameinstanceref _nodeid_2))
    (`/Game/GameDesign/Luis/Level_Proto/MapaJuego/Blueprints/BPI_MapNode.RefreshVisualState` _array_element_2 _returnvalue_2)
    (`KismetSystemLibrary.PrintString` (`|GetEnumeratorNameAsString` _returnvalue_2))
    (`KismetSystemLibrary.PrintString` (`KismetStringLibrary.Conv_NameToString` _nodeid_2))))

(fn `IsNodeAccessible`
  (params (NodeRef :type "/Game/GameDesign/Luis/Level_Proto/MapaJuego/Blueprints/BP_MapNode_Base Object Reference"))
  (returns (IsAccesible :type Boolean))
  (bind _returnvalue (`/Game/GameDesign/Luis/Level_Proto/MapaJuego/Blueprints/BP_GI_MapZ1.GetNodeState` (`self.GameInstanceRef`) (`/Game/GameDesign/Luis/Level_Proto/MapaJuego/Blueprints/BP_MapNode_Base.NodeID` NodeRef)))
  (return (or (`|EnumEquality` _returnvalue "NewEnumerator2") (`|EnumEquality` _returnvalue "NewEnumerator1"))))

(fn `LockOtherAvailableNodes`
  (params (ChosenNode :type "/Game/GameDesign/Luis/Level_Proto/MapaJuego/Blueprints/BP_MapNode_Base Object Reference"))
  (bind _gameinstanceref (`self.GameInstanceRef`))
  (bind _values (`BlueprintMapLibrary.Map_Values` (`self.RegsiteredNodes`)))
  (for _array_element _values
    (if (!= _array_element ChosenNode)
      (bind _nodeid (`/Game/GameDesign/Luis/Level_Proto/MapaJuego/Blueprints/BP_MapNode_Base.NodeID` _array_element))
      (bind _returnvalue (`/Game/GameDesign/Luis/Level_Proto/MapaJuego/Blueprints/BP_GI_MapZ1.GetNodeState` _gameinstanceref _nodeid))
      (if (`|EnumEquality` _returnvalue "NewEnumerator1")
        (`/Game/GameDesign/Luis/Level_Proto/MapaJuego/Blueprints/BP_GI_MapZ1.SaveNodeState` _gameinstanceref _nodeid "NewEnumerator4")
        (`/Game/GameDesign/Luis/Level_Proto/MapaJuego/Blueprints/BP_MapNode_Base.RefreshVisualState` _array_element "NewEnumerator0")))))

(fn `RegisterNode`
  (params (NodeId :type Name) (NodeRef :type "/Game/GameDesign/Luis/Level_Proto/MapaJuego/Blueprints/BP_MapNode_Base Object Reference"))
  (`BlueprintMapLibrary.Map_Add` (`self.RegsiteredNodes`) NodeId NodeRef))

(fn `SelectNode`
  (params (NodeRef :type "/Game/GameDesign/Luis/Level_Proto/MapaJuego/Blueprints/BP_MapNode_Base Object Reference"))
  (bind _nodeid (`/Game/GameDesign/Luis/Level_Proto/MapaJuego/Blueprints/BP_MapNode_Base.NodeID` NodeRef))
  (bind _isaccesible (`self.IsNodeAccessible` NodeRef))
  (if _isaccesible
    (`/Game/GameDesign/Luis/Level_Proto/MapaJuego/Blueprints/BP_GI_MapZ1.SaveNodeState` (`self.GameInstanceRef`) _nodeid "NewEnumerator2")
    (`self.LockOtherAvailableNodes` NodeRef)
    (message `/Game/GameDesign/Luis/Level_Proto/MapaJuego/Blueprints/BPI_MapNode.RefreshVisualState` NodeRef "NewEnumerator2")
    (`/Game/GameDesign/Luis/Level_Proto/MapaJuego/Blueprints/BP_GI_MapZ1.SetCurrentNode` (`self.GameInstanceRef`) _nodeid)
    (message `/Game/GameDesign/Luis/Level_Proto/MapaJuego/Blueprints/BPI_MapNode.TryEnterNode` NodeRef)
    (else
      (`KismetSystemLibrary.PrintString` "Cuidao"))))

(fn `UnlockNextNodes`
  (params (NodeRef :type "/Game/GameDesign/Luis/Level_Proto/MapaJuego/Blueprints/BP_MapNode_Base Object Reference"))
  (bind _gameinstanceref (`self.GameInstanceRef`))
  (for _array_element (`/Game/GameDesign/Luis/Level_Proto/MapaJuego/Blueprints/BP_MapNode_Base.NextNodes` NodeRef)
    (bind _nodeid (`/Game/GameDesign/Luis/Level_Proto/MapaJuego/Blueprints/BP_MapNode_Base.NodeID` _array_element))
    (bind _returnvalue (`/Game/GameDesign/Luis/Level_Proto/MapaJuego/Blueprints/BP_GI_MapZ1.GetNodeState` _gameinstanceref _nodeid))
    (if (`|EnumEquality` _returnvalue "NewEnumerator0")
      (`/Game/GameDesign/Luis/Level_Proto/MapaJuego/Blueprints/BP_GI_MapZ1.SaveNodeState` _gameinstanceref _nodeid "NewEnumerator1"))))

(fn `UserConstructionScript`)