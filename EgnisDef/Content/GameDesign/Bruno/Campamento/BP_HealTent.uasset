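; BP_HealTent is a heal tent interactable for the camp that opens the camp HUD's interact panel.
; On interaction it reuses an existing top-level WBP_CampHUD or creates one and adds it to the viewport.
; It passes itself and its interact info to the panel.
; The graph holds no healing logic, and its OnCampOptionChosen call is unconnected.
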(event `self.Interactable.OnInteracted`
  (bind _foundwidgets (`WidgetBlueprintLibrary.GetAllWidgetsOfClass` "/Game/GameDesign/Bruno/Campamento/WBP_CampHUD.WBP_CampHUD_C"))
  (if (> (`KismetArrayLibrary.Array_Length` _foundwidgets) 0)
    (`/Game/GameDesign/Bruno/Campamento/WBP_CampHUD.ShowInteractPanel` (`KismetArrayLibrary.Array_Get` _foundwidgets) self (`self.IntertactInfo`))
    (else
      (bind _returnvalue (`|CreateWidget` "/Game/GameDesign/Bruno/Campamento/WBP_CampHUD.WBP_CampHUD_C" (`GameplayStatics.GetPlayerController` 0)))
      (`UserWidget.AddToViewport` _returnvalue 0)
      (`/Game/GameDesign/Bruno/Campamento/WBP_CampHUD.ShowInteractPanel` _returnvalue self (`self.IntertactInfo`)))))

(fn `UserConstructionScript`)