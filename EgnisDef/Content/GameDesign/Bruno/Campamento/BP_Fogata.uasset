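; BP_Fogata is a camp campfire actor that opens an interaction panel when the player interacts with it.
; On interaction it reuses an existing top-level WBP_CampHUD, or creates one for the first player controller, then shows the panel with itself as target and its InteractInfo.
; OnCampOptionChosen switches on an ActionId but has no actions wired, and OnComponentActivated is empty.
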(event `self.Interactable.OnInteracted`
  (bind _foundwidgets (`WidgetBlueprintLibrary.GetAllWidgetsOfClass` "/Game/GameDesign/Bruno/Campamento/WBP_CampHUD.WBP_CampHUD_C"))
  (if (> (`KismetArrayLibrary.Array_Length` _foundwidgets) 0)
    (`/Game/GameDesign/Bruno/Campamento/WBP_CampHUD.ShowInteractPanel` (`KismetArrayLibrary.Array_Get` _foundwidgets) self (`self.InteractInfo`))
    (else
      (bind _returnvalue (`|CreateWidget` "/Game/GameDesign/Bruno/Campamento/WBP_CampHUD.WBP_CampHUD_C" (`GameplayStatics.GetPlayerController` 0)))
      (`UserWidget.AddToViewport` _returnvalue 0)
      (`/Game/GameDesign/Bruno/Campamento/WBP_CampHUD.ShowInteractPanel` _returnvalue self (`self.InteractInfo`)))))

(event `self.Interactable.OnComponentActivated`
  (params (Component :type "ActorComponent Object Reference") (bReset :type Boolean)))

(event `/Game/GameDesign/Bruno/Campamento/BPI_CampInteractable.OnCampOptionChosen`
  (params (ActionId :type Name))
  (switch `name` ActionId))

(fn `UserConstructionScript`)