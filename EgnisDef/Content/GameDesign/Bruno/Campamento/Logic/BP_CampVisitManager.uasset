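; Camp visit manager that tracks and enforces what the player can do during one campfire visit: restore one flame and heal one hero.
; Healing repeats on that hero with per-attempt odds from an editable list; a failed coin flip ends healing for the visit.
; State changes go through RunProgressionSubsystem and fire OnVisitChanged, with helpers for wounded heroes and crack-material amount.
; Returning delegates to the level's MapEncounterExit; BeginPlay can seed a test run.
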(event `self.ReceiveBeginPlay`
  ;[0.6 0.35 0.1] GESTOR DE LA VISITA AL CAMPAMENTO: guarda que se ha hecho en esta visita (1 llama, 1 personaje sanado). Lo crea BFL_Camp.GetVisitManager si no esta colocado en el nivel.
  (`self.CreateTestRunIfNeeded`)
  (`self.ResetVisit`))

(fn `CanHealHero`
  (params (HeroId :type Name))
  (returns (bCan :type Boolean))
  ;[0.6 0.35 0.1] Se puede sanar si: la moneda no ha fallado, es el MISMO personaje de esta visita (solo 1 por visita) y tiene heridas.
  (return (and (and (not (`self.bSanacionTerminada`)) (or (== (`self.HeroeSanado`) "None") (== (`self.HeroeSanado`) HeroId))) (> (`self.GetHeroWoundCount` HeroId) 0))))

(fn `CanRestoreFlame`
  (returns (bCan :type Boolean))
  (return (and (not (`self.bLlamaRecuperada`)) (< (`RunProgressionSubsystem.GetCampfire` (`self.GetRun`)) (`self.LlamaMaxima`)))))

(fn `CreateTestRunIfNeeded`
  (locals (Heroes :type "Array of HeroDataAsset Object Reference"))
  (bind _run (`self.GetRun`))
  (bind _heroesheridosdeprueba (`self.HeroesHeridosDePrueba`))
  ;[0.6 0.35 0.1] SOLO PARA PROBAR EL CAMPAMENTO SUELTO: crea una run con HeroesHeridosDePrueba (cada uno con sus Heridas) y quita 1 llama. En el juego real la run ya viene del mapa.
  (if (and (`self.bCrearRunDePrueba`) (not (`RunProgressionSubsystem.IsRunActive` _run)))
    (for _array_element _heroesheridosdeprueba
      (`KismetArrayLibrary.Array_Add` (`local.Heroes`) (`.Hero_2_1AFA072045C2C63DC80E6D90722FF15A` (break `/Game/GameDesign/Bruno/Campamento/Logic/S_TestWoundedHero` _array_element))))
    (`RunProgressionSubsystem.StartNewRun` _run (`local.Heroes`) (`self.MazoDePrueba`))
    (for _array_element_2 _heroesheridosdeprueba
      (bind (_hero _heridas) (break `/Game/GameDesign/Bruno/Campamento/Logic/S_TestWoundedHero` _array_element_2))
      (for _ (range 1 (+ _heridas 1))
        (`RunProgressionSubsystem.AddRandomWound` _run (`RunProgressionSubsystem.GetHeroId` _hero))))
    (`RunProgressionSubsystem.LoseCampfire` _run)
    (return)))

(fn `GetCrackAmount`
  (params (HeroId :type Name))
  (returns (Amount :type "Float (double-precision)"))
  (return (`KismetMathLibrary.FClamp` (/ (`KismetMathLibrary.Conv_IntToDouble` (`self.GetHeroWoundCount` HeroId)) (`KismetMathLibrary.Conv_IntToDouble` (`self.MaxHeridas`))))))

(fn `GetHealChance`
  (returns (Chance :type "Float (double-precision)"))
  (bind _probabilidadessanacion (`self.ProbabilidadesSanacion`))
  (bind _numsanaciones (`self.NumSanaciones`))
  (return (`KismetMathLibrary.SelectFloat` (/ (`KismetMathLibrary.Conv_IntToDouble` (`KismetArrayLibrary.Array_Get` _probabilidadessanacion _numsanaciones)) 100.0) 0.0 (`KismetArrayLibrary.Array_IsValidIndex` _probabilidadessanacion _numsanaciones))))

(fn `GetHeroWoundCount`
  (params (HeroId :type Name))
  (returns (Wounds :type Integer))
  (return (`KismetArrayLibrary.Array_Length` (`.Wounds` (break `HeroRuntimeData` (`RunProgressionSubsystem.GetHeroState` (`self.GetRun`) HeroId))))))

(fn `GetRun`
  (returns (Run :type "RunProgressionSubsystem Object Reference"))
  ;[0.6 0.35 0.1] Acceso unico a la mochila de la run (RunProgressionSubsystem). Usar siempre este getter.
  (return (subsystem `RunProgressionSubsystem`)))

(fn `GetWoundedHeroes`
  (returns (Heroes :type "Array of HeroRuntimeData Structure"))
  (locals (Resultado :type "Array of HeroRuntimeData Structure"))
  ;[0.6 0.35 0.1] Heroes desbloqueados con al menos 1 herida (lo que muestra el Taller del carpintero).
  (`KismetArrayLibrary.Array_Clear` (`local.Resultado`))
  (for _array_element (`RunProgressionSubsystem.GetUnlockedHeroes` (`self.GetRun`))
    (if (> (`KismetArrayLibrary.Array_Length` (`.Wounds` (break `HeroRuntimeData` _array_element))) 0)
      (`KismetArrayLibrary.Array_Add` (`local.Resultado`) _array_element)))
  (return (`local.Resultado`)))

(fn `ResetVisit`
  (set `self.NumSanaciones` 0)
  (set `self.HeroeSanado` "None")
  (set `self.bSanacionTerminada` false)
  (set `self.bLlamaRecuperada` false)
  (`self.OnVisitChanged`)
  (return))

(fn `RestoreFlame`
  (returns (bRestored :type Boolean))
  ;[0.6 0.35 0.1] RECUPERAR LLAMA: +1 llama (RestoreCampfire) una sola vez por visita.
  (if (`self.CanRestoreFlame`)
    (`RunProgressionSubsystem.RestoreCampfire` (`self.GetRun`) 1)
    (set `self.bLlamaRecuperada` true)
    (`self.OnVisitChanged`)
    (return true)
    (else
      (return false))))

(fn `ReturnToMap`
  (returns (bOk :type Boolean))
  ;[0.6 0.35 0.1] VOLVER AL MAPA: usa el AMapEncounterExit (C++) del nivel: completa la casilla actual y abre ReturnMap.
  (bind _returnvalue (`GameplayStatics.GetActorOfClass` "/Script/EgnisDef.MapEncounterExit"))
  (bind _asmap_encounter_exit (cast `MapEncounterExit` _returnvalue)
    (:`then`
      (bind _returnvalue_2 (`MapEncounterExit.CompleteAndReturn` _asmap_encounter_exit))
      (return _returnvalue_2))
    (:`CastFailed`
      (`KismetSystemLibrary.PrintString` "Campamento: no hay ningun MapEncounterExit en el nivel, no se puede volver al mapa")
      (return false))))

(fn `TryHealHero`
  (params (HeroId :type Name))
  (returns (bHealed :type Boolean) (bCoinFailed :type Boolean))
  ;[0.6 0.35 0.1] SANAR: 1a sanacion gratis. Despues se tira una moneda con GetHealChance. Exito -> HealOneWound (herida mas antigua) y el personaje queda fijado. Fallo -> se acaba la sanacion de esta visita.
  (if (`self.CanHealHero` HeroId)
    (if (`KismetMathLibrary.RandomBoolWithWeight` (`self.GetHealChance`))
      (bind _returnvalue (`RunProgressionSubsystem.HealOneWound` (`self.GetRun`) HeroId))
      (set `self.NumSanaciones` (+ (`self.NumSanaciones`) 1))
      (set `self.HeroeSanado` HeroId)
      (`self.OnVisitChanged`)
      (return _returnvalue false)
      (else
        (set `self.bSanacionTerminada` true)
        (`self.OnVisitChanged`)
        (return false true)))
    (else
      (return false false))))

(fn `UserConstructionScript`)