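; BP_CaveMenuButton is a clickable in-world main menu button with a painted text label shown through a widget component.
; Construction and BeginPlay push LabelText into the WBP_CavePaintLabel widget.
; Cursor-over events set a hover flag, and Tick eases it with FInterpTo to slide the pivot along local X and drive the label material's Glow.
; Clicking finds the BP_MainMenuController in the level and passes it the button's ActionId.
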(event `self.ReceiveBeginPlay`
  ;[0.6 0.35 0.1] Label + hover animation
  (`self.RefreshLabel`))

(event `self.ReceiveTick`
  (params (DeltaSeconds :type "Float (single-precision)"))
  ;[0.6 0.35 0.1] Label + hover animation
  (`self.UpdateHover` DeltaSeconds))

(event `self.ReceiveActorBeginCursorOver`
  ;[0.6 0.35 0.1] Mouse interaction (needs click / mouse-over events on the PlayerController)
  (`self.SetHovered` true))

(event `self.ReceiveActorEndCursorOver`
  ;[0.6 0.35 0.1] Mouse interaction (needs click / mouse-over events on the PlayerController)
  (`self.SetHovered` false))

(event `self.ReceiveActorOnClicked`
  (params (ButtonPressed :type "Key Structure"))
  ;[0.6 0.35 0.1] Mouse interaction (needs click / mouse-over events on the PlayerController)
  (`self.Activate`))

(fn `Activate`
  (bind _returnvalue (`GameplayStatics.GetActorOfClass` (`self.ControllerClass`)))
  (bind _asbp_main_menu_controller (cast `/Game/GameDesign/Bruno/MainMenu/Blueprints/BP_MainMenuController` _returnvalue))
  (`/Game/GameDesign/Bruno/MainMenu/Blueprints/BP_MainMenuController.HandleMenuAction` _asbp_main_menu_controller (`self.ActionId`)))

(fn `RefreshLabel`
  (bind _aswbp_cave_paint_label (cast `/Game/GameDesign/Bruno/MainMenu/Widgets/WBP_CavePaintLabel` (`WidgetComponent.GetUserWidgetObject` (`self.Label`))))
  (`/Game/GameDesign/Bruno/MainMenu/Widgets/WBP_CavePaintLabel.SetLabel` _aswbp_cave_paint_label (`KismetTextLibrary.Conv_StringToText` (`self.LabelText`))))

(fn `SetHovered`
  (params (bNewHovered :type Boolean))
  (set `self.bHovered` bNewHovered))

(fn `UpdateHover`
  (params (DeltaTime :type "Float (double-precision)"))
  (bind _returnvalue (`WidgetComponent.GetMaterialInstance` (`self.Label`)))
  (bind _output_get (set `self.HoverAlpha` (`KismetMathLibrary.FInterpTo` (`self.HoverAlpha`) (`KismetMathLibrary.SelectFloat` 1.0 0.0 (`self.bHovered`)) DeltaTime (`self.HoverSpeed`))))
  (`SceneComponent.K2_SetRelativeLocation` (`self.Pivot`) (`KismetMathLibrary.MakeVector` (* _output_get (`self.HoverOffset`))) false false)
  (if (`KismetSystemLibrary.IsValid` _returnvalue)
    (`MaterialInstanceDynamic.SetScalarParameterValue` _returnvalue "Glow" (* _output_get (`self.GlowMax`)))))

(fn `UserConstructionScript`
  (`self.RefreshLabel`))