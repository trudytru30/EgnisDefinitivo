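; Main menu controller that acts as the view target and runs the Start and Quit actions with camera fades.
; On BeginPlay it points the player's view at itself, enables game-and-UI input and fades in from black.
; HandleMenuAction maps an action ID to an event, ignoring requests once a transition has started.
; Each action fades out picture and audio, waits the fade duration, then opens the gameplay level or quits.
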(event `self.ReceiveBeginPlay`
  ;[0.6 0.35 0.1] Setup: fixed camera, mouse input, fade in
  (`self.SetupView`)
  (`self.FadeCamera` 1.0))

(event `StartGame`
  ;[0.6 0.35 0.1] Menu actions
  (set `self.bTransitioning` true)
  (`self.FadeCamera` 0.0 1.0)
  (`KismetSystemLibrary.Delay` (`self.FadeDuration`))
  (`GameplayStatics.OpenLevel` (`self.GameplayLevel`)))

(event `QuitGame`
  ;[0.6 0.35 0.1] Menu actions
  (set `self.bTransitioning` true)
  (`self.FadeCamera` 0.0 1.0)
  (`KismetSystemLibrary.Delay` (`self.FadeDuration`))
  (`KismetSystemLibrary.QuitGame` (`GameplayStatics.GetPlayerController` 0) "Quit"))

(fn `FadeCamera`
  (params (FromAlpha :type "Float (double-precision)") (ToAlpha :type "Float (double-precision)"))
  (`PlayerCameraManager.StartCameraFade` :`self` (`GameplayStatics.GetPlayerCameraManager` 0) :`FromAlpha` FromAlpha :`ToAlpha` ToAlpha :`Duration` (`self.FadeDuration`) :`bShouldFadeAudio` true :`bHoldWhenFinished` true))

(fn `HandleMenuAction`
  (params (ActionId :type String))
  (if (`self.bTransitioning`)
    _
    (elif (`KismetStringLibrary.EqualEqual_StrStr` ActionId "Start")
      (`self.StartGame`)
      (elif (`KismetStringLibrary.EqualEqual_StrStr` ActionId "Quit")
        (`self.QuitGame`)))))

(fn `SetupView`
  (bind _returnvalue (`GameplayStatics.GetPlayerController` 0))
  (`PlayerController.SetViewTargetWithBlend` _returnvalue self 0.0 "VTBlend_Linear" 0.0 false)
  (`WidgetBlueprintLibrary.SetInputMode_GameAndUIEx` _returnvalue null "DoNotLock" false))

(fn `UserConstructionScript`)