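; Fire light controller for the main menu that gives a fire's light an irregular flicker and a slight positional wander.
; BeginPlay stores the light's home position and randomizes the noise offset.
; Each Tick, layered Perlin noise drives smoothed intensity, with a slower or faster gust term, plus jitter around home.
; SetFireActive toggles the Fire component and eases intensity toward zero when off, while StopFire animates attenuation radius through a timeline.
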(event `self.ReceiveBeginPlay`
  (`self.InitFire`))

(event `StopFire`
  (bind (_direction _light) (`Timeline|Timeline`)
    (:`Update`
      (`LocalLightComponent.SetAttenuationRadius` (`self.FireLight`) _light))))

(event `self.ReceiveTick`
  (params (DeltaSeconds :type "Float (single-precision)"))
  ;[0.6 0.35 0.1] irregular intensity wandering position
  (`self.UpdateLight` DeltaSeconds))

(fn `ComputeFlicker`
  (returns (Multiplier :type "Float (double-precision)"))
  (bind _returnvalue (* (`self.NoiseTime`) (`self.FlickerSpeed`)))
  (return (+ (+ (* (+ (* (`KismetMathLibrary.PerlinNoise1D` _returnvalue) 0.65) (* (`KismetMathLibrary.PerlinNoise1D` (+ (* _returnvalue 2.37) 31.7)) 0.35)) (`self.FlickerAmount`)) (* (`KismetMathLibrary.PerlinNoise1D` (+ (* (`self.NoiseTime`) (`self.GustSpeed`)) 73.1)) (`self.GustAmount`))) 1.0)))

(fn `InitFire`
  (set `self.LightHome` (`SceneComponent.K2_GetComponentLocation` (`self.FireLight`)))
  (set `self.NoiseTime` (`KismetMathLibrary.RandomFloatInRange` 0.0 100.0))
  (set `self.CurrentIntensity` (`self.BaseIntensity`))
  (`LocalLightComponent.SetAttenuationRadius` (`self.FireLight`) (`self.AttenuationRadius`)))

(fn `SetFireActive`
  (params (bActive :type Boolean))
  (set `self.bFireActive` bActive)
  (`ActorComponent.SetActive` (`self.Fire`) bActive false))

(fn `UpdateLight`
  (params (DeltaTime :type "Float (double-precision)"))
  (bind _returnvalue (* (`self.NoiseTime`) (`self.JitterSpeed`)))
  (set `self.NoiseTime` (+ (`self.NoiseTime`) DeltaTime))
  (bind _output_get (set `self.CurrentIntensity` (`KismetMathLibrary.FInterpTo` (`self.CurrentIntensity`) (* (* (`self.BaseIntensity`) (`self.ComputeFlicker`)) (`KismetMathLibrary.SelectFloat` 1.0 0.0 (`self.bFireActive`))) DeltaTime (`self.SmoothSpeed`))))
  (`LightComponent.SetIntensity` (`self.FireLight`) _output_get)
  (`SceneComponent.K2_SetWorldLocation` (`self.FireLight`) (+ (`self.LightHome`) (* (`KismetMathLibrary.MakeVector` (`KismetMathLibrary.PerlinNoise1D` (+ _returnvalue 11.3)) (`KismetMathLibrary.PerlinNoise1D` (+ _returnvalue 47.9)) (`KismetMathLibrary.PerlinNoise1D` (+ _returnvalue 89.1))) (`self.JitterRadius`))) false false))

(fn `UserConstructionScript`)