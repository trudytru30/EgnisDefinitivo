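; Off-screen studio actor that renders the mesh shown by WBP_ModelInspector into a transparent-clear render target via a show-only SceneCapture.
; It frames each piece from its bounds, plays a damped cosine bounce drop, recaptures briefly, and supports rotation and clamped zoom.
; Queued portrait requests share the same capture, pausing animation to render into caller-supplied targets over two ticks each, then restore the inspected piece.
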(event `self.ReceiveBeginPlay`
  ;[0.1 0.25 0.45] Inicio: crear la textura de render y encuadrar
  (`self.SetupCapture`)
  (`self.FrameAndCapture`))

(event `InspectMesh`
  (params (Mesh :type "StaticMesh Object Reference"))
  (bind _previewmesh (`self.PreviewMesh`))
  ;[0.15 0.35 0.15] Mostrar una pieza (lo llama WBP_ModelInspector)
  (set `self.InspectedMesh` Mesh)
  (set `self.InspectedMaterial` null)
  (`StaticMeshComponent.SetStaticMesh` _previewmesh Mesh)
  (`PrimitiveComponent.SetMaterial` _previewmesh 0 null)
  (`self.FrameAndCapture`))

(event `InspectMeshWithMaterial`
  (params (Mesh :type "StaticMesh Object Reference") (Material :type "MaterialInterface Object Reference"))
  (bind _previewmesh (`self.PreviewMesh`))
  ;[0.15 0.35 0.15] Mostrar una pieza (lo llama WBP_ModelInspector)
  (set `self.InspectedMesh` Mesh)
  (set `self.InspectedMaterial` Material)
  (`StaticMeshComponent.SetStaticMesh` _previewmesh Mesh)
  (`PrimitiveComponent.SetMaterial` _previewmesh 0 Material)
  (`self.FrameAndCapture`))

(event `FrameAndCapture`
  ;[0.45 0.3 0.1] Encuadrar la pieza y lanzar la animación de caída
  (`self.RestartRecapture`)
  (`self.FacePieceToCamera`)
  (`self.FitCameraToPiece`)
  (`self.StartDrop`)
  (`self.ApplyDistanceAndCapture`))

(event `ApplyDistanceAndCapture`
  ;[0.35 0.15 0.4] Cámara y controles del jugador (rotar / zoom)
  (`self.MoveCameraToDistance`)
  (`SceneCaptureComponent2D.CaptureScene` (`self.Capture`)))

(event `RotatePiece`
  (params (DeltaYaw :type "Float (double-precision)") (DeltaPitch :type "Float (double-precision)"))
  ;[0.35 0.15 0.4] Cámara y controles del jugador (rotar / zoom)
  (`SceneComponent.K2_AddWorldRotation` (`self.Pivot`) (`KismetMathLibrary.MakeRotator` 0.0 DeltaPitch DeltaYaw) false false)
  (`SceneCaptureComponent2D.CaptureScene` (`self.Capture`)))

(event `ZoomPiece`
  (params (Amount :type "Float (double-precision)"))
  ;[0.35 0.15 0.4] Cámara y controles del jugador (rotar / zoom)
  (`self.ApplyZoom` Amount)
  (`self.ApplyDistanceAndCapture`))

(event `self.ReceiveTick`
  (params (DeltaSeconds :type "Float (single-precision)"))
  ;[0.4 0.1 0.1] Cada frame: animación de caída y recaptura
  (if (> (`KismetArrayLibrary.Array_Length` (`self.PortraitMeshes`)) 0)
    (`self.ProcessPortraitStep`)
    (else
      (`self.UpdateDropAnimation` DeltaSeconds)
      (`self.UpdateRecapture` DeltaSeconds))))

(event `QueuePortrait`
  (params (Mesh :type "StaticMesh Object Reference") (Target :type "TextureRenderTarget2D Object Reference"))
  ;[0.45 0.4 0.1] Retratos: la cuadrícula pide un retrato por héroe (se hacen de uno en uno en el Tick)
  (`KismetArrayLibrary.Array_Add` (`self.PortraitMeshes`) Mesh)
  (`KismetArrayLibrary.Array_Add` (`self.PortraitTargets`) Target))

(fn `ApplyZoom`
  (params (Amount :type "Float (double-precision)"))
  (bind _basedistance (`self.BaseDistance`))
  (set `self.Distance` (`KismetMathLibrary.FClamp` (- (`self.Distance`) (* Amount (* _basedistance 0.1))) (* _basedistance 0.4) (* _basedistance 2.5))))

(fn `FacePieceToCamera`
  (bind _facingyaw (`self.FacingYaw`))
  (`SceneComponent.K2_SetRelativeRotation` (`self.Pivot`) (`KismetMathLibrary.MakeRotator` 0.0 0.0 (`KismetMathLibrary.SelectFloat` (+ _facingyaw 180.0) _facingyaw (`KismetArrayLibrary.Array_Contains` (`self.FlippedMeshes`) (`StaticMeshComponent.StaticMesh` (`self.PreviewMesh`))))) false false))

(fn `FitCameraToPiece`
  (bind _previewmesh (`self.PreviewMesh`))
  (bind _staticmesh (`StaticMeshComponent.StaticMesh` _previewmesh))
  (bind (_origin _boxextent _sphereradius) (`KismetMathLibrary.BreakBoxSphereBounds` (`StaticMesh.GetBounds` _staticmesh)))
  (bind _returnvalue (* _sphereradius 4.2))
  (`/Engine/EditorBlueprintResources/StandardMacros.IsValid` _staticmesh
    (:`Is Valid`
      (`SceneComponent.K2_SetRelativeLocation` _previewmesh (* _origin -1.0) false false)
      (set `self.BaseDistance` _returnvalue)
      (set `self.Distance` _returnvalue))))

(fn `MoveCameraToDistance`
  (`SceneComponent.K2_SetRelativeLocation` (`self.Capture`) (`KismetMathLibrary.MakeVector` (* (`self.Distance`) -1.0)) false false))

(fn `ProcessPortraitStep`
  (bind _portraittargets (`self.PortraitTargets`))
  (bind _capture (`self.Capture`))
  (bind _inspectedmesh (`self.InspectedMesh`))
  (bind _previewmesh (`self.PreviewMesh`))
  (bind _portraitmeshes (`self.PortraitMeshes`))
  (if (== (`self.PortraitStep`) 0)
    (`StaticMeshComponent.SetStaticMesh` (`self.PreviewMesh`) (`KismetArrayLibrary.Array_Get` _portraitmeshes))
    (`self.FacePieceToCamera`)
    (`self.FitCameraToPiece`)
    (`SceneComponent.K2_SetRelativeLocation` (`self.Pivot`) (0.0 0.0 0.0) false false)
    (`self.MoveCameraToDistance`)
    (set `self.PortraitStep` 1)
    (else
      (set `SceneCaptureComponent2D.TextureTarget` (`KismetArrayLibrary.Array_Get` _portraittargets) _capture)
      (`SceneCaptureComponent2D.CaptureScene` _capture)
      (set `SceneCaptureComponent2D.TextureTarget` (`self.RenderTarget`) _capture)
      (`KismetArrayLibrary.Array_Remove` _portraitmeshes)
      (`KismetArrayLibrary.Array_Remove` _portraittargets)
      (set `self.PortraitStep` 0)
      (if (== (`KismetArrayLibrary.Array_Length` _portraitmeshes) 0)
        (`/Engine/EditorBlueprintResources/StandardMacros.IsValid` _inspectedmesh
          (:`Is Valid`
            (`StaticMeshComponent.SetStaticMesh` _previewmesh _inspectedmesh)
            (`PrimitiveComponent.SetMaterial` _previewmesh 0 (`self.InspectedMaterial`))
            (`self.FrameAndCapture`)))))))

(fn `RestartRecapture`
  (set `self.RecaptureTimeLeft` (`self.RecaptureDuration`)))

(fn `SetupCapture`
  (bind _capture (`self.Capture`))
  (bind _returnvalue (`KismetRenderingLibrary.CreateRenderTarget2D` 2048 2048 "RTF_RGBA16f" (struct) true))
  (set `self.RenderTarget` _returnvalue)
  (set `SceneCaptureComponent2D.TextureTarget` _returnvalue _capture)
  (`SceneCaptureComponent.ShowOnlyComponent` _capture (`self.PreviewMesh`)))

(fn `StartDrop`
  (bind _returnvalue (* (`self.BaseDistance`) (`self.DropHeightFactor`)))
  (set `self.DropHeight` _returnvalue)
  (set `self.DropElapsed` 0.0)
  (set `self.DropProgress` 0.0)
  (`SceneComponent.K2_SetRelativeLocation` (`self.Pivot`) (`KismetMathLibrary.MakeVector` 0.0 0.0 _returnvalue) false false))

(fn `UpdateDropAnimation`
  (params (DeltaSeconds :type "Float (double-precision)"))
  (bind _dropelapsed (`self.DropElapsed`))
  (bind _dropprogress (`self.DropProgress`))
  (if (< _dropelapsed (`self.DropDuration`))
    (set `self.DropElapsed` (+ _dropelapsed DeltaSeconds))
    (set `self.DropProgress` (`KismetMathLibrary.FClamp` (/ (`self.DropElapsed`) (`self.DropDuration`))))
    (`SceneComponent.K2_SetRelativeLocation` (`self.Pivot`) (`KismetMathLibrary.MakeVector` 0.0 0.0 (* (* (`KismetMathLibrary.Abs` (`KismetMathLibrary.Cos` (* _dropprogress (* (+ (`KismetMathLibrary.Conv_IntToDouble` (`self.BounceCount`)) 0.5) 3.14159265)))) (`KismetMathLibrary.MultiplyMultiply_FloatFloat` (- 1.0 _dropprogress) (`self.BounceDamping`))) (`self.DropHeight`))) false false)))

(fn `UpdateRecapture`
  (params (DeltaSeconds :type "Float (double-precision)"))
  (bind _recapturetimeleft (`self.RecaptureTimeLeft`))
  (if (> _recapturetimeleft 0.0)
    (`SceneCaptureComponent2D.CaptureScene` (`self.Capture`))
    (set `self.RecaptureTimeLeft` (- _recapturetimeleft DeltaSeconds))))

(fn `UserConstructionScript`)