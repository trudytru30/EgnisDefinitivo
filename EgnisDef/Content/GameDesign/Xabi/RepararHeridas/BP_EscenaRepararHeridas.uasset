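; Scene actor for the wound repair screen, which opens the WBP_RepararHeridas widget on BeginPlay and switches the player to UI-only input with a visible cursor.
; For standalone testing, if no run is active and CrearRunDePrueba is set, it first builds a test run through RunProgressionSubsystem from HeroesDePrueba, gives each hero random wounds and loses a campfire.
; In normal play the run already comes from the map.
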(event `self.ReceiveBeginPlay`
  (bind _returnvalue (`GameplayStatics.GetPlayerController` 0))
  (bind _returnvalue_2 (subsystem `RunProgressionSubsystem`))
  ;[0.3 0.15 0.35] ESCENA REPARAR HERIDAS. 1) Solo para probar la escena suelta: si no hay run activa y bCrearRunDePrueba=true, crea una run con HeroesDePrueba, 2 heridas aleatorias a cada uno y pierde 1 llama. En el juego real la run ya viene del mapa. 2) Crea WBP_RepararHeridas y pone el raton en modo UI.
  (if (and (not (`RunProgressionSubsystem.IsRunActive` (subsystem `RunProgressionSubsystem`))) (`self.bCrearRunDePrueba`))
    (`RunProgressionSubsystem.StartNewRun` (subsystem `RunProgressionSubsystem`) (`self.HeroesDePrueba`) (`|MakeArray` null :!type "BaseCard Object Reference"))
    (for _array_element (`self.HeroesDePrueba`)
      (bind _returnvalue_3 (`RunProgressionSubsystem.GetHeroId` _array_element))
      (`RunProgressionSubsystem.AddRandomWound` _returnvalue_2 _returnvalue_3)
      (`RunProgressionSubsystem.AddRandomWound` _returnvalue_2 _returnvalue_3))
    (`RunProgressionSubsystem.LoseCampfire` _returnvalue_2))
  (bind _returnvalue_4 (`|CreateWidget` "/Game/GameDesign/Xabi/RepararHeridas/WBP_RepararHeridas.WBP_RepararHeridas_C" _returnvalue))
  (`UserWidget.AddToViewport` _returnvalue_4 0)
  (set `PlayerController.bShowMouseCursor` true _returnvalue)
  (`WidgetBlueprintLibrary.SetInputMode_UIOnlyEx` _returnvalue _returnvalue_4))

(fn `UserConstructionScript`)