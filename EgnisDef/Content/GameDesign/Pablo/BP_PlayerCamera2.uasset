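; BP_PlayerCamera2 is a player camera that offers zoom and horizontal rotation through Enhanced Input.
; The zoom action adds scaled input to the camera's orthographic width, clamped between minimum and maximum limits, rather than changing arm length.
; The move action adds scaled input to the spring arm's world yaw, passing its relative pitch and roll through, so it rotates rather than pans.
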(event `EnhancedInput|/Game/Inputs/IA_CameraZoom`
  (params (ActionValue :type "Float (double-precision)") (ElapsedSeconds :type "Float (double-precision)") (TriggeredSeconds :type "Float (double-precision)") (InputAction :type "InputAction Object Reference" :default "/Game/Inputs/IA_CameraZoom.IA_CameraZoom"))
  (bind _camera (`self.Camera`))
  ; Zoom Cámara
  (:`Triggered`
    (`CameraComponent.SetOrthoWidth` _camera (`KismetMathLibrary.FClamp` (+ (* ActionValue (`self.ZoomSpeed`)) (`CameraComponent.OrthoWidth` _camera)) (`self.MinZoom`) (`self.MaxZoom`)))))

(event `EnhancedInput|/Game/Inputs/IA_CameraMove`
  (params (ActionValue :type "Float (double-precision)") (ElapsedSeconds :type "Float (double-precision)") (TriggeredSeconds :type "Float (double-precision)") (InputAction :type "InputAction Object Reference" :default "/Game/Inputs/IA_CameraMove.IA_CameraMove"))
  (bind (_returnvalue_roll _returnvalue_pitch _returnvalue_yaw) (`KismetMathLibrary.BreakRotator` (`SceneComponent.K2_GetComponentRotation` (`self.SpringArm`))))
  (bind (_relativerotation_roll _relativerotation_pitch) (`KismetMathLibrary.BreakRotator` (`SceneComponent.RelativeRotation` (`self.SpringArm`))))
  ; Movimiento Cámara
  (:`Triggered`
    (`SceneComponent.K2_SetWorldRotation` (`self.SpringArm`) (`KismetMathLibrary.MakeRotator` _relativerotation_roll _relativerotation_pitch (+ (* ActionValue (`self.CameraSpeed`)) _returnvalue_yaw)) false false)))

(fn `UserConstructionScript`)