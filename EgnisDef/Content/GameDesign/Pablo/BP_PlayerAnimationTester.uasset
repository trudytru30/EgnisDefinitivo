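; Test actor for previewing procedural player death and attack animations on a static mesh.
; BeginPlay runs DieAnimation, whose timeline drives the mesh's relative location in X/Z and its rotation, with sweep and teleport enabled.
; AttackAnimation uses a second timeline to move the mesh in X/Y and rotate it without sweep, but nothing in this graph calls it.
; Both keep the mesh's current scale.
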(event `self.ReceiveBeginPlay`
  (`self.DieAnimation`))

(event `DieAnimation`
  (bind (_direction _position _rotation) (`Timeline|DeathAnimation` :`NewTime` 2.0)
    (:`Update`
      (`SceneComponent.K2_SetRelativeTransform` (`self.StaticMesh`) (`KismetMathLibrary.MakeTransform` (`KismetMathLibrary.MakeVector` (.x _position) 0.0 (.z _position)) (`KismetMathLibrary.MakeRotator` (.x _rotation) (.z _rotation) (.y _rotation)) (`SceneComponent.RelativeScale3D` (`self.StaticMesh`))) true true))))

(event `AttackAnimation`
  (bind (_direction _position _rotation) (`Timeline|AttackAnim` :`NewTime` 0.2)
    (:`Update`
      (`SceneComponent.K2_SetRelativeTransform` (`self.StaticMesh`) (`KismetMathLibrary.MakeTransform` (`KismetMathLibrary.MakeVector` (.x _position) (.y _position)) (`KismetMathLibrary.MakeRotator` (.x _rotation) (.y _rotation) (.z _rotation)) (`SceneComponent.RelativeScale3D` (`self.StaticMesh`))) false false))))

(fn `UserConstructionScript`)