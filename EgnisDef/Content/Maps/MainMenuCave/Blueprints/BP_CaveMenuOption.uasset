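; BP_CaveMenuOption is a clickable 3D menu option for the cave main menu.
; On BeginPlay it sets its ClickBox to BlockAll collision, and cursor events swap the TargetText actor between hover and normal scale.
; A click branches on the Action value to open LevelToOpen for Play or quit the game for Quit.
; Any other action only prints a Spanish placeholder saying options are not yet implemented.
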(event `self.ReceiveBeginPlay`
  (`PrimitiveComponent.SetCollisionProfileName` (`self.ClickBox`) "BlockAll" true))

(event `self.ReceiveActorOnClicked`
  (params (ButtonPressed :type "Key Structure"))
  (bind _action (`self.Action`))
  (if (== _action "Play")
    (`GameplayStatics.OpenLevel` (`self.LevelToOpen`))
    (elif (== _action "Quit")
      (`KismetSystemLibrary.QuitGame` null "Quit")
      (else
        (`KismetSystemLibrary.PrintString` "Opciones: pendiente de implementar")))))

(event `self.ReceiveActorBeginCursorOver`
  (`self.SetActorScale3D` (`self.TargetText`) (`self.HoverScale`)))

(event `self.ReceiveActorEndCursorOver`
  (`self.SetActorScale3D` (`self.TargetText`) (`self.NormalScale`)))

(fn `UserConstructionScript`)