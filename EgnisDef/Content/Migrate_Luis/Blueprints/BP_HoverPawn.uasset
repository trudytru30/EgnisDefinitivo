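; BP_HoverPawn is a mouse-draggable piece that drops onto actors tagged "Tile".
; Cursor hover activates smoke and a green outline overlay material.
; Clicking stores the start location and makes the mesh ignore Visibility, so Tick's cursor trace moves the pawn along whatever lies beneath.
; On release it jumps to the hit tile's location or back to its start, then clears effects and restores blocking.
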(event `self.ReceiveBeginPlay`
  ;[0.8594 0.8594 0.8594 0.5] Effectos Overlay
  (`ActorComponent.Deactivate` (`self.Smoke`))
  (`MeshComponent.SetOverlayMaterial` (`self.Mesh`) null))

(event `self.ReceiveActorBeginCursorOver`
  ;[0.8594 0.8594 0.8594 0.5] Effectos Overlay
  (`ActorComponent.Activate` (`self.Smoke`) true)
  (`MeshComponent.SetOverlayMaterial` (`self.Mesh`) "/Game/Migrate_Luis/Materials/Outline/MI_OutlineGreen.MI_OutlineGreen"))

(event `self.ReceiveActorEndCursorOver`
  ;[0.8594 0.8594 0.8594 0.5] Effectos Overlay
  (`ActorComponent.Deactivate` (`self.Smoke`))
  (`MeshComponent.SetOverlayMaterial` (`self.Mesh`) null))

(event `self.ReceiveActorOnClicked`
  (params (ButtonPressed :type "Key Structure"))
  ; Cazao
  (set `self.StartLocation` (`self.K2_GetActorLocation`))
  (set `self.Dragging` true)
  (`PrimitiveComponent.SetCollisionResponseToChannel` (`self.Mesh`) "ECC_Visibility" "ECR_Ignore"))

(event `self.ReceiveTick`
  (params (DeltaSeconds :type "Float (single-precision)"))
  (bind _returnvalue (`GameplayStatics.GetPlayerController` 0))
  (bind _mesh (`self.Mesh`))
  (bind (_hitresult _returnvalue_2) (`PlayerController.GetHitResultUnderCursorByChannel` _returnvalue "TraceTypeQuery1" true))
  (bind (_bblockinghit _binitialoverlap _time _distance _location _impactpoint _normal _impactnormal _physmat _hitactor) (`GameplayStatics.BreakHitResult` _hitresult))
  ; Cazao
  (if (`self.Dragging`)
    (if (`PlayerController.IsInputKeyDown` _returnvalue "LeftMouseButton")
      (if _returnvalue_2
        (`self.K2_SetActorLocation` _location))
      (else
        (if (`self.ActorHasTag` _hitactor "Tile")
          (`self.K2_SetActorLocation` (`self.K2_GetActorLocation` _hitactor))
          (else
            (`self.K2_SetActorLocation` (`self.StartLocation`))))
        (set `self.Dragging` false)
        (`ActorComponent.Deactivate` (`self.Smoke`))
        (`MeshComponent.SetOverlayMaterial` _mesh null)
        (`PrimitiveComponent.SetCollisionResponseToChannel` _mesh "ECC_Visibility" "ECR_Block")))))

(fn `UserConstructionScript`)