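; BP_BlueShield is a one-shot bubble shield effect: a sphere that grows, freezes, flashes and shrinks away.
; BeginPlay hides the sphere at zero scale and gives it a dynamic bubble material.
; ActivateShield, also bound to the H key, chains four timelines, each starting when the previous finishes: scale-in, freeze ramp, implosion flash, scale-out.
; Setter functions push freeze and void progress into material parameters, and Activated is never reset, blocking replays.
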(event `self.ReceiveBeginPlay`
  (bind _sphere (`self.Sphere`))
  (`SceneComponent.SetRelativeScale3D` _sphere (0.0 0.0 0.0))
  (bind _returnvalue (`PrimitiveComponent.CreateDynamicMaterialInstance` _sphere 0 "/Game/Migrate_Luis/Effects/MERN/M_BubbleWers.M_BubbleWers" "None"))
  (set `self.DynMat` _returnvalue)
  (`MaterialInstanceDynamic.SetScalarParameterValue` _returnvalue "FreezeProgress" (`self.FreezeProgress`))
  (`MaterialInstanceDynamic.SetScalarParameterValue` _returnvalue "ImplosionFlash" (`self.VoidProgress`)))

(event `ActivateShield`
  (if (not (`self.bActivated`))
    (set `self.bActivated` true)
    (bind (_direction _alpha) (`Timeline|ScaleInTimeLine`)
      (:`Update`
        (bind _returnvalue (`KismetMathLibrary.VLerp` (0.0 0.0 0.0) (2.0 2.0 2.0) _alpha))
        (`SceneComponent.SetRelativeScale3D` (`self.Sphere`) _returnvalue))
      (:`Finished`
        (bind (_direction_2 _progress) (`Timeline|FreezeRampTimeline`)
          (:`Update`
            (`self.SetFreezeProgress` (`KismetMathLibrary.Lerp` 0.0 (`self.FreezeTarget`) _progress)))
          (:`Finished`
            (bind (_direction_3 _voidprogress) (`Timeline|VoidTimeLine`)
              (:`Update`
                (`self.SetVoidProgress` (`KismetMathLibrary.Lerp` 0.0 (`self.VoidTarget`) _voidprogress)))
              (:`Finished`
                (bind (_direction_4 _alpha_2) (`Timeline|ScaleTimeLineReverese`)
                  (:`Update`
                    (`SceneComponent.SetRelativeScale3D` (`self.Sphere`) (`KismetMathLibrary.VLerp` _returnvalue (0.0 0.0 0.0) _alpha_2))))))))))))

(event `Key|H`
  (params (Key :type "Key Structure"))
  (:`Pressed`
    (`self.ActivateShield`)))

(fn `SetFreezeProgress`
  (params (NewValue :type "Float (double-precision)"))
  (bind _output_get (set `self.FreezeProgress` NewValue))
  (`MaterialInstanceDynamic.SetScalarParameterValue` (`self.DynMat`) "FreezeProgress" _output_get))

(fn `SetVoidProgress`
  (params (NewValue :type "Float (double-precision)"))
  (bind _output_get (set `self.VoidProgress` NewValue))
  (`MaterialInstanceDynamic.SetScalarParameterValue` (`self.DynMat`) "ImplosionFlash" _output_get))

(fn `UserConstructionScript`)