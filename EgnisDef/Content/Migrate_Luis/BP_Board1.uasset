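; Tile board actor that draws a grid and highlights destination and range tiles.
; The construction script rebuilds Tiles as instanced meshes over BoardSizeX by BoardSizeY, placed with TileToWorldCenter and scaled by TileVisualSize.
; MostrarMarcador moves one destination marker, colored lime if valid or red if not, while MostrarAlcance fills a second instanced set from a tile list.
; Markers sit at slightly staggered heights above the board, and Ocultar functions hide or clear them.
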(fn `MostrarAlcance`
  (params (Casillas :type "Array of TileCoord Structure"))
  (bind _returnvalue (* (`self.TileVisualSize`) 0.009))
  (`InstancedStaticMeshComponent.ClearInstances` (`self.MarcadoresAlcance`))
  (for _array_element Casillas
    (`InstancedStaticMeshComponent.AddInstance` (`self.MarcadoresAlcance`) (`KismetMathLibrary.MakeTransform` (+ (`self.TileToWorldCenter` _array_element) (0.0 0.0 1.5)) (struct) (`KismetMathLibrary.MakeVector` _returnvalue _returnvalue 1.0)) true)))

(fn `MostrarMarcador`
  (params (Casillas :type "TileCoord Structure") (Valida :type Boolean))
  (bind _marcador_destino (`self.Marcador Destino`))
  (`SceneComponent.K2_SetWorldLocation` _marcador_destino (+ (`self.TileToWorldCenter` Casillas) (0.0 0.0 2.0)) false false)
  (if Valida
    (`PrimitiveComponent.SetMaterial` _marcador_destino 0 "/Game/Materials/Lima.Lima")
    (else
      (`PrimitiveComponent.SetMaterial` _marcador_destino 0 "/Game/Materials/RedEnemyW.RedEnemyW")))
  (`SceneComponent.SetHiddenInGame` _marcador_destino false false))

(fn `OcultarAlcance`
  (`InstancedStaticMeshComponent.ClearInstances` (`self.MarcadoresAlcance`)))

(fn `OcultarMarcador`
  (`SceneComponent.SetHiddenInGame` (`self.Marcador Destino`) true false))

(fn `UserConstructionScript`
  (bind _returnvalue (* (`self.TileVisualSize`) 0.01))
  (`InstancedStaticMeshComponent.ClearInstances` (`self.Tiles`))
  (for _index (range (`self.BoardSizeX`))
    (for _index_2 (range (`self.BoardSizeY`))
      (`InstancedStaticMeshComponent.AddInstance` (`self.Tiles`) (`KismetMathLibrary.MakeTransform` (+ (`self.TileToWorldCenter` (make `TileCoord` _index _index_2)) (0.0 0.0 1.0)) (struct) (`KismetMathLibrary.MakeVector` _returnvalue _returnvalue 1.0)) true))))