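; BP_NodeDifficulty is a clickable map node that displays a difficulty level and leads into the L_TestPartida test level.
; Clicking its sphere toggles ClickOn and shifts the sphere vertically, lowering it and passing the node to MapManagerRef.SelectNode, or raising it back on the alternate click.
; The construction script writes DifficultyLevel to the DifLevel text.
; TryEnterNode opens the hardcoded level regardless of difficulty.
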(event `self.Sphere.OnClicked`
  (params (TouchedComponent :type "PrimitiveComponent Object Reference") (ButtonPressed :type "Key Structure"))
  (bind _sphere (`self.Sphere`))
  ; Button Sistem
  (if (`self.Click On`)
    (`SceneComponent.K2_AddWorldOffset` _sphere (0.0 0.0 25.0) false false)
    (set `self.Click On` false)
    (else
      (`SceneComponent.K2_AddWorldOffset` _sphere (0.0 0.0 -25.0) false false)
      (set `self.Click On` true)
      (`/Game/Media/Level_Proto/MapaJuego/Blueprints/BP_MapManager.SelectNode` (`self.MapManagerRef`) self))))

(event `/Game/Media/Level_Proto/MapaJuego/Blueprints/BPI_MapNode.TryEnterNode`
  ; Button Sistem
  (`GameplayStatics.OpenLevel` "L_TestPartida"))

(fn `UserConstructionScript`
  (`TextRenderComponent.K2_SetText` (`self.DifLevel`) (`KismetTextLibrary.Conv_IntToText` (`self.DifficultyLevel`))))