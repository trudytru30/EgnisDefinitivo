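; Player character for the map level that shows a fixed overhead-style map camera and pans it with mouse drag.
; On BeginPlay it adds the drag input mapping, blends the view to the actor tagged Camera_01, and enables cursor, click events and Game-and-UI input.
; IA_DragCamera sets Dragging, which nothing clears, letting IA_MouseDelta move the camera in world X/Y with sweep.
; An older mouse-position drag and a plane-intersection calculation remain unused.
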(event `self.ReceiveBeginPlay`
  (bind _returnvalue (`GameplayStatics.GetPlayerController` 0))
  ; Game Cick and Ui
  (set `PlayerController.bShowMouseCursor` true _returnvalue)
  (`EnhancedInputSubsystemInterface.AddMappingContext` (pcsubsystem `EnhancedInputLocalPlayerSubsystem` _returnvalue) "/Game/Media/Level_Proto/MapaJuego/InputActions/IMC_CameraDrag.IMC_CameraDrag" 0 (struct))
  (bind _asplayer_controller (cast `PlayerController` (`self.GetController`)))
  (bind _outactors (`GameplayStatics.GetAllActorsWithTag` "Camera_01"))
  (bind _output_get (set `self.FixedCamera` (`|GetArrayItem` _outactors)))
  (`PlayerController.SetViewTargetWithBlend` _asplayer_controller _output_get 1.0 "VTBlend_Linear" 0.0 false)
  (set `PlayerController.bShowMouseCursor` true _asplayer_controller)
  (`WidgetBlueprintLibrary.SetInputMode_GameAndUIEx` _asplayer_controller null)
  (set `PlayerController.bEnableClickEvents` true _asplayer_controller))

(event `EnhancedInput|/Game/Media/Level_Proto/MapaJuego/InputActions/IA_DragCamera`
  (params (ActionValue :type Boolean) (ElapsedSeconds :type "Float (double-precision)") (TriggeredSeconds :type "Float (double-precision)") (InputAction :type "InputAction Object Reference" :default "/Game/Media/Level_Proto/MapaJuego/InputActions/IA_DragCamera.IA_DragCamera"))
  (:`Started`
    (set `self.bDragging` true)))

(event `self.ReceiveTick`
  (params (DeltaSeconds :type "Float (single-precision)")))

(event `EnhancedInput|/Game/Media/Level_Proto/MapaJuego/InputActions/IA_MouseDelta`
  (params (ActionValue :type "Vector Structure") (ElapsedSeconds :type "Float (double-precision)") (TriggeredSeconds :type "Float (double-precision)") (InputAction :type "InputAction Object Reference" :default "/Game/Media/Level_Proto/MapaJuego/InputActions/IA_MouseDelta.IA_MouseDelta"))
  (bind _dragsensitivity (`self.DragSensitivity`))
  (bind (_x _y) (`KismetMathLibrary.BreakVector2D` (`KismetMathLibrary.Conv_VectorToVector2D` ActionValue)))
  (:`Triggered`
    (if (`self.bDragging`)
      (`self.K2_AddActorWorldOffset` (`self.FixedCamera`) (`KismetMathLibrary.MakeVector` (* _y _dragsensitivity -1.0) (* _dragsensitivity _x -1.0)) true false))))

(fn `UserConstructionScript`)