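; BP_GI_MapZ1 is a Game Instance that holds node progress for a game map.
; A NodeStates map stores an enum state per node ID, with getters and setters that fall back to the first enum value for unknown nodes.
; On Init it moves the "Diff1" node from that default state to the second one.
; It also tracks the current node ID through a simple setter and getter.
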(event `self.ReceiveInit`
  (bind _returnvalue (`self.GetNodeState` "Diff1"))
  (if (`|EnumEquality` _returnvalue "NewEnumerator0")
    (`self.SaveNodeState` "Diff1" "NewEnumerator1")))

(fn `GetCurrentNode`
  (returns (OutputName :type Name))
  (return (`self.CurrentNodeID`)))

(fn `GetNodeState`
  (params (NodeID :type Name))
  (returns (ReturnValue :type "/Game/Media/Level_Proto/MapaJuego/Enum/ENodeState Enum"))
  (bind _nodestates (`self.NodeStates`))
  (if (`BlueprintMapLibrary.Map_Contains` _nodestates NodeID)
    (return (`BlueprintMapLibrary.Map_Find` _nodestates NodeID))
    (else
      (return "NewEnumerator0"))))

(fn `SaveNodeState`
  (params (NodeID :type Name) (NewState :type "/Game/Media/Level_Proto/MapaJuego/Enum/ENodeState Enum" :default "NewEnumerator0"))
  (`BlueprintMapLibrary.Map_Add` (`self.NodeStates`) NodeID NewState)
  (return))

(fn `SetCurrentNode`
  (params (NewNodeID :type Name))
  (set `self.CurrentNodeID` NewNodeID)
  (return))