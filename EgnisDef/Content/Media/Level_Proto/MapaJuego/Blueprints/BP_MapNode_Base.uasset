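; BP_MapNode_Base is the base actor for a node on the game map, shown as a sphere whose color reflects its state.
; On BeginPlay it caches the first BP_MapManager in the level and creates a dynamic instance of M_Button on the sphere.
; RefreshVisualState sets that material's NodeColor parameter to a distinct color for each state: locked, available, current, completed or discarded.
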(event `/Game/Media/Level_Proto/MapaJuego/Blueprints/BPI_MapNode.RefreshVisualState`
  (params (NewState :type "/Game/Media/Level_Proto/MapaJuego/Enum/ENodeState Enum" :default "NewEnumerator0"))
  (bind _dynmaterial (`self.DynMaterial`))
  (switch `/Game/Media/Level_Proto/MapaJuego/Enum/ENodeState` NewState
    (:`NewEnumerator0`
      (`MaterialInstanceDynamic.SetVectorParameterValue` _dynmaterial "NodeColor" (struct :`R` 0.052083 :`G` 0.052083 :`B` 0.052083 :`A` 1.0)))
    (:`NewEnumerator1`
      (`MaterialInstanceDynamic.SetVectorParameterValue` _dynmaterial "NodeColor" (struct :`R` 0.786458 :`G` 0.283996 :`B` 0.033371 :`A` 1.0)))
    (:`NewEnumerator2`
      (`MaterialInstanceDynamic.SetVectorParameterValue` _dynmaterial "NodeColor" (struct :`R` 1.0 :`G` 0.96327 :`B` 0.026042 :`A` 1.0)))
    (:`NewEnumerator3`
      (`MaterialInstanceDynamic.SetVectorParameterValue` _dynmaterial "NodeColor" (struct :`G` 1.0 :`B` 0.043707 :`A` 1.0)))
    (:`NewEnumerator4`
      (`MaterialInstanceDynamic.SetVectorParameterValue` _dynmaterial "NodeColor" (struct :`A` 1.0)))))

(event `self.ReceiveBeginPlay`
  ; Dynamic Material
  (bind _outactors (`GameplayStatics.GetAllActorsOfClass` "/Game/Media/Level_Proto/MapaJuego/Blueprints/BP_MapManager.BP_MapManager_C"))
  (set `self.MapManagerRef` (`|GetArrayItem` _outactors))
  (bind _returnvalue (`PrimitiveComponent.CreateDynamicMaterialInstance` (`self.Sphere`) 0 "/Game/Media/Level_Proto/MapaJuego/Buttons/M_Button.M_Button" "None"))
  (set `self.DynMaterial` _returnvalue)
  (`PrimitiveComponent.SetMaterial` (`self.Sphere`) 0 (`self.DynMaterial`)))

(fn `UserConstructionScript`)