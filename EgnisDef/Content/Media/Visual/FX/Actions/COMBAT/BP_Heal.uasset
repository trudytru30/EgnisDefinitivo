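; BP_Heal is a heal visual effect actor with a beam and a Niagara-style NSHEAL effect, triggered by ActiveHeal or the B key.
; ActiveHeal activates NSHEAL and plays the BeamAnim timeline, which widens the beam and scales up the effect.
; After a short hold, it deactivates NSHEAL and reverses the timeline to shrink both.
; The Activated flag blocks retriggering until then and stops the reversed timeline from looping.
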(event `self.ReceiveBeginPlay`
  (`self.EnableInput` (`GameplayStatics.GetPlayerController` 0))
  (`SceneComponent.SetRelativeScale3D` (`self.Beam`) (0.0 0.0 0.0)))

(event `ActiveHeal`
  (if (not (`self.bActivated`))
    (set `self.bActivated` true)
    (`ActorComponent.Activate` (`self.NS_HEAL`) true)
    (bind (_direction _alpha) (`Timeline|BeamAnim` :!label _label)
      (:`Update`
        (`SceneComponent.SetRelativeScale3D` (`self.Beam`) (`KismetMathLibrary.VLerp` (0.0 0.0 21.2075) (4.5625 4.5625 21.2075) _alpha))
        (`SceneComponent.SetRelativeScale3D` (`self.NS_HEAL`) (`KismetMathLibrary.VLerp` (0.0 0.0 0.0) (0.77 0.77 0.77) _alpha)))
      (:`Finished`
        (if (`self.bActivated`)
          (`KismetSystemLibrary.Delay` 1.0)
          (set `self.bActivated` false)
          (`ActorComponent.Deactivate` (`self.NS_HEAL`))
          (goto _label :!via `Reverse`))))))

(event `Key|B`
  (params (Key :type "Key Structure"))
  (:`Pressed`
    (`self.ActiveHeal`)))

(fn `UserConstructionScript`)