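; BP_Shield is a shield effect actor whose sphere is scaled up from zero when activated.
; It enables input from player 0 on BeginPlay, and the C key calls ActiveShield and prints a debug "Hello".
; ActiveShield plays a Timeline that lerps the sphere scale, or reverses it while the Activated flag is set.
; The flag clears after a short delay once the Timeline finishes, without itself shrinking the sphere.
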(event `self.ReceiveBeginPlay`
  (`self.EnableInput` (`GameplayStatics.GetPlayerController` 0))
  (`SceneComponent.SetRelativeScale3D` (`self.Sphere`) (0.0 0.0 0.0)))

(event `ActiveShield`
  (if (not (`self.Activated`))
    (set `self.Activated` true)
    (bind (_direction _alpha) (`Timeline|Timeline` :!label _label)
      (:`Update`
        (`SceneComponent.SetRelativeScale3D` (`self.Sphere`) (`KismetMathLibrary.VLerp` (0.0 0.0 0.0) (4.0 4.0 4.0) _alpha)))
      (:`Finished`
        (`KismetSystemLibrary.Delay` 1.0)
        (set `self.Activated` false)))
    (else
      (goto _label :!via `Reverse`))))

(event `Key|C`
  (params (Key :type "Key Structure"))
  (:`Pressed`
    (`self.ActiveShield`)
    (`KismetSystemLibrary.PrintText` "Hello")))

(fn `UserConstructionScript`)