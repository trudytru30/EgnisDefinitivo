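; Impact frames manager actor that plays an impact effect at its location when key 1 is pressed, with input enabled for the first player on BeginPlay.
; Impact spawns the Niagara impact frame system, optionally adding a world camera shake and an extra VFX system, each gated by a flag.
; An optional repeat flag loops the whole sequence on a two-second delay.
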(event `self.ReceiveBeginPlay`
  (`self.EnableInput` (`GameplayStatics.GetPlayerController` 0)))

(event `Key|One`
  (params (Key :type "Key Structure"))
  (:`Pressed`
    (`self.Impact`)))

(event `Impact`
  (bind _returnvalue (`self.K2_GetActorLocation`))
  (`|ExecutionSequence` :!label _label
    (:`then_0`
      (if (`self.doShake`)
        (`GameplayStatics.PlayWorldCameraShake` (`self.Shake`) _returnvalue 0.0 100000.0 0.0)))
    (:`then_1`
      (`NiagaraFunctionLibrary.SpawnSystemAtLocation` (`self.ImpactFrameSystem`) _returnvalue))
    (:`then_2`
      (if (`self.doExtra`)
        (`NiagaraFunctionLibrary.SpawnSystemAtLocation` (`self.Extra VFX`) _returnvalue)))
    (:`then_3`
      (if (`self.doRepeat`)
        (`KismetSystemLibrary.Delay` 2.0)
        (goto _label)))))

(fn `UserConstructionScript`)