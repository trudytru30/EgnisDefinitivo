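; BP_Fire is a one-shot fire effect actor that pairs a scaling sphere with a spark effect (NSChispa).
; It starts hidden with sparks off, and pressing E triggers Implosion, guarded so it fires only once, plus a debug print.
; One timeline grows the sphere to full scale, then the sparks activate and, after a short delay, a second timeline shrinks it away.
; The sparks are never deactivated afterward, as that node is unconnected.
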(event `self.ReceiveBeginPlay`
  (`self.EnableInput` (`GameplayStatics.GetPlayerController` 0))
  (`SceneComponent.SetRelativeScale3D` (`self.Sphere1`) (0.0 0.0 0.0))
  (`ActorComponent.Deactivate` (`self.NS_Chispa`)))

(event `Implosion`
  (if (not (`self.Activated`))
    (set `self.Activated` true)
    (bind (_direction _alpha) (`Timeline|Timeline`)
      (:`Update`
        (`SceneComponent.SetRelativeScale3D` (`self.Sphere1`) (`KismetMathLibrary.VLerp` (0.0 0.0 0.0) (1.0 1.0 1.0) _alpha)))
      (:`Finished`
        (`ActorComponent.Activate` (`self.NS_Chispa`) true)
        (`KismetSystemLibrary.Delay` 2.0)
        (bind (_direction_2 _alpha_2) (`Timeline|Timeline_1`)
          (:`Update`
            (`SceneComponent.SetRelativeScale3D` (`self.Sphere1`) (`KismetMathLibrary.VLerp` (1.0 1.0 1.0) (0.0 0.0 0.0) _alpha_2))))))))

(event `Key|E`
  (params (Key :type "Key Structure"))
  (:`Pressed`
    (`self.Implosion`)
    (`KismetSystemLibrary.PrintText` "Hello")))

(fn `UserConstructionScript`)