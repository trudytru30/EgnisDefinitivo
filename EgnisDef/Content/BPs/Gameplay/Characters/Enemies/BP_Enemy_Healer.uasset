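; Healer enemy character Blueprint whose graph handles only a spinning attack mark indicator; no healing logic appears here.
; BeginPlay binds the MarkSpin movement component to AttackMark and hides it.
; SetAttackMark toggles the mark's visibility and activates or deactivates its spin to match.
; An unconnected leftover chain would also place the mark just above the capsule's bottom.
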(event `self.ReceiveBeginPlay`
  (bind _attackmark (`self.AttackMark`))
  ; Rotation and Visbility
  (`MovementComponent.SetUpdatedComponent` (`self.MarkSpin`) _attackmark)
  (`SceneComponent.SetHiddenInGame` _attackmark true false))

(event `/Game/BPs/Gameplay/Characters/Enemies/BPI_AttackMark.SetAttackMark`
  (params (Visible :type Boolean))
  (bind _markspin (`self.MarkSpin`))
  ; SetAttackMArk
  (`SceneComponent.SetHiddenInGame` (`self.AttackMark`) (not Visible) false)
  (if Visible
    (`ActorComponent.Activate` _markspin false)
    (else
      (`ActorComponent.Deactivate` _markspin))))

(fn `UserConstructionScript`)