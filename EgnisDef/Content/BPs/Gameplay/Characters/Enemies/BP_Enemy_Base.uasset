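; Base enemy Blueprint that handles overhead health bar, highlight outline and spinning attack mark.
; On BeginPlay it gives each static mesh except the mark a per-enemy dynamic overlay material and places the bar above the tallest mesh.
; Attribute-change events refresh the bar and debug texts.
; ActualizarResaltado switches outline brightness, thickness and text visibility for mouse hover, while Tick interpolates bar opacity; SetAttackMark toggles the mark and stamps its material start time.
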(event `self.ReceiveBeginPlay`
  (bind _attackmark (`self.AttackMark`))
  ; Rotation and Visbility
  (`self.AplicarContorno`)
  (`self.AjustarAlturaBarra`)
  (`AbilityAsync_WaitAttributeChanged.WaitForAttributeChanged` null (struct :`AttributeName` "Health" :`Attribute` "/Script/EgnisDef.HealthAttributeSet:Health" :`AttributeOwner` "/Script/CoreUObject.Class'/Script/EgnisDef.HealthAttributeSet'")
    (:`then`
      _)
    (:`Changed`
      (`self.HealthBarLogic`)))
  (`MovementComponent.SetUpdatedComponent` (`self.MarkSpin`) _attackmark)
  (`SceneComponent.SetHiddenInGame` _attackmark true false)
  (`KismetSystemLibrary.DelayUntilNextTick`)
  (`self.HealthBarLogic`))

(event `/Game/BPs/Gameplay/Characters/Enemies/BPI_AttackMark.SetAttackMark`
  (params (Visible :type Boolean))
  (bind _markspin (`self.MarkSpin`))
  (bind _attackmark (`self.AttackMark`))
  ; SetAttackMArk
  (if (and Visible (`SceneComponent.bHiddenInGame` _attackmark))
    (bind _returnvalue (`PrimitiveComponent.CreateDynamicMaterialInstance` _attackmark 0 null "None"))
    (`MaterialInstanceDynamic.SetScalarParameterValue` _returnvalue "StartTime" (`KismetSystemLibrary.GetGameTimeInSeconds`)))
  (`SceneComponent.SetHiddenInGame` (`self.AttackMark`) (not Visible) false)
  (if Visible
    (`ActorComponent.Activate` _markspin false)
    (else
      (`ActorComponent.Deactivate` _markspin))))

(event `self.ReceiveTick`
  (params (DeltaSeconds :type "Float (single-precision)"))
  ;[0.25 0.45 0.9] Cada frame: fundido suave de la barra de vida (aparece y desaparece con el raton)
  (`self.ActualizarFundidoBarra` DeltaSeconds))

(fn `ActualizarFundidoBarra`
  (params (DeltaSeconds :type "Float (double-precision)"))
  (bind _healthbar (`self.HealthBar`))
  (bind _returnvalue (`WidgetComponent.GetUserWidgetObject` _healthbar))
  ;[0.25 0.45 0.9] 1. Acercar la opacidad poco a poco a la objetivo (VelocidadFundidoBarra)
  (bind _output_get (set `self.OpacidadBarra` (`KismetMathLibrary.FInterpTo` (`self.OpacidadBarra`) (`self.OpacidadBarraObjetivo`) DeltaSeconds (`self.VelocidadFundidoBarra`))))
  (if (`KismetSystemLibrary.IsValid` _returnvalue)
    ;[0.9 0.15 0.1] 2. Aplicarla al widget; si es casi 0 se oculta el componente del todo
    (`Widget.SetRenderOpacity` _returnvalue _output_get)
    (`SceneComponent.SetVisibility` _healthbar (> _output_get 0.01) false)))

(fn `ActualizarResaltado`
  (params (bResaltado :type Boolean))
  (bind _contornodinamico (`self.ContornoDinamico`))
  ;[0.25 0.45 0.9] 1. Barra de vida: marcar si debe verse (1) o no (0); el fundido suave lo hace ActualizarFundidoBarra en el Tick. Textos de vida: visibles solo con el raton encima
  (set `self.OpacidadBarraObjetivo` (`KismetMathLibrary.SelectFloat` 1.0 0.0 bResaltado))
  (`SceneComponent.SetVisibility` (`self.maxhealth_test`) bResaltado false)
  (`SceneComponent.SetVisibility` (`self.currenthealth_test`) bResaltado false)
  ;[0.9 0.15 0.1] 2. Contorno rojo: mas brillo y grosor con el raton encima (si ya se ha creado)
  (if (`KismetSystemLibrary.IsValid` _contornodinamico)
    (`MaterialInstanceDynamic.SetVectorParameterValue` _contornodinamico "Color" (* (`self.ColorContorno`) (`KismetMathLibrary.SelectFloat` (`self.BrilloHover`) (`self.BrilloNormal`) bResaltado)))
    (`MaterialInstanceDynamic.SetScalarParameterValue` _contornodinamico "Grosor" (`KismetMathLibrary.SelectFloat` (`self.GrosorHover`) (`self.GrosorNormal`) bResaltado))))

(fn `AjustarAlturaBarra`
  (bind _alturamaximamodelo (`self.AlturaMaximaModelo`))
  ;[0.25 0.45 0.9] 1. Buscar el punto mas alto de los modelos del enemigo (sin la marca de ataque)
  (set `self.AlturaMaximaModelo` (.z (`self.K2_GetActorLocation`)))
  (for _array_element (`self.K2_GetComponentsByClass` "/Script/Engine.StaticMeshComponent")
    (if (`self.EsMallaDelEnemigo` _array_element)
      (bind (_origin _boxextent) (`KismetSystemLibrary.GetComponentBounds` _array_element))
      (set `self.AlturaMaximaModelo` (`KismetMathLibrary.FMax` _alturamaximamodelo (+ (.z _origin) (.z _boxextent))))))
  ;[0.9 0.15 0.1] 2. Colocar la barra centrada sobre el enemigo, MargenAlturaBarra por encima
  (`SceneComponent.K2_SetWorldLocation` (`self.HealthBar`) (`KismetMathLibrary.MakeVector` (.x (`self.K2_GetActorLocation`)) (.y (`self.K2_GetActorLocation`)) (+ _alturamaximamodelo (`self.MargenAlturaBarra`))) false false))

(fn `AplicarContorno`
  (bind _returnvalue (`KismetMaterialLibrary.CreateDynamicMaterialInstance` (`self.MaterialContorno`)))
  ;[0.9 0.15 0.1] 1. Crear el contorno rojo propio de este enemigo (para poder cambiar su brillo sin afectar a los demas)
  (bind _output_get (set `self.ContornoDinamico` _returnvalue))
  ;[0.25 0.45 0.9] 2. Ponerlo como Overlay Material en cada modelo del enemigo (no en la marca de ataque)
  (for _array_element (`self.K2_GetComponentsByClass` "/Script/Engine.StaticMeshComponent")
    (if (`self.EsMallaDelEnemigo` _array_element)
      (`MeshComponent.SetOverlayMaterial` _array_element _output_get)))
  ;[0.6 0.6 0.6] 3. Estado inicial: sin resaltar y barra oculta
  (`self.ActualizarResaltado` false))

(fn `EsMallaDelEnemigo`
  (params (Componente :type "StaticMeshComponent Object Reference"))
  (returns (EsMalla :type Boolean))
  (return (not (`KismetStringLibrary.Contains` (`KismetSystemLibrary.GetObjectName` Componente) "AttackMark"))))

(fn `HealthBarLogic`
  (bind _returnvalue (`self.GetCurrentHealth`))
  (bind _returnvalue_2 (`self.GetMaxHealth`))
  (bind _returnvalue_3 (/ _returnvalue _returnvalue_2))
  (bind _aswb_health_bar (cast `/Game/Media/Visual/UI/MenuElements/WB_HealthBar` (`WidgetComponent.GetWidget` (`self.HealthBar`))))
  (`ProgressBar.SetPercent` (`/Game/Media/Visual/UI/MenuElements/WB_HealthBar.HealthProgresBar` _aswb_health_bar) _returnvalue_3)
  (`KismetSystemLibrary.PrintString` (`KismetStringLibrary.Conv_DoubleToString` _returnvalue_3))
  (`TextRenderComponent.K2_SetText` (`self.maxhealth_test`) (`KismetTextLibrary.Conv_DoubleToText` _returnvalue "HalfToEven"))
  (`TextRenderComponent.K2_SetText` (`self.currenthealth_test`) (`KismetTextLibrary.Conv_DoubleToText` _returnvalue_2 "HalfToEven")))

(fn `UserConstructionScript`)