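; Allied unit on the tile board, handling its movement queries and visual feedback.
; On spawn it snaps to its tile, drops in and fires a landing wave through a material parameter collection; jumps follow a Timeline-driven parabola.
; GAS attribute listeners flash the model white on health or shield loss, using a retriggerable delay.
; Tick drives a crack overlay from health unless hidden by rule; rotating heal/shield marks and a smoke-aura outline show status.
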(event `Update Marks`
  (`MovementComponent.SetUpdatedComponent` (`self.RotatingMovement`) (`self.HealMark`))
  (`MovementComponent.SetUpdatedComponent` (`self.RotatingMovement1`) (`self.ShieldMark`)))

(event `self.ReceiveBeginPlay`
  ; Seteo Base
  (`self.EscucharDano`)
  (`self.StartCracks`)
  (`self.Update Marks`)
  (`KismetSystemLibrary.Delay` 0.0)
  ;; Onda Seteo Base
  (bind _returnvalue (`self.SetCurrentTile` (`Board.WorldPointToTile` (`self.Board`) (`self.K2_GetActorLocation`))))
  (if _returnvalue
    (`self.SnapToCurrentTile` false))
  (bind _output_get (set `self.CaidaFin` (`self.K2_GetActorLocation`)))
  (bind _output_get_2 (set `self.CaidaInicio` (+ _output_get (`KismetMathLibrary.MakeVector` 0.0 0.0 (`self.AlturaCaida`)))))
  (`self.K2_SetActorLocation` _output_get_2)
  (`KismetSystemLibrary.MoveComponentTo` (`self.RootComponent`) (`KismetMathLibrary.MakeVector` (.x _output_get) (.y _output_get) (.z _output_get)) (`self.K2_GetActorRotation`) false true 0.5)
  (`self.LanzarOnda` _output_get))

(event `SaltarA`
  (params (Inicio :type "Vector Structure") (Destino :type "Vector Structure"))
  (bind _saltofin (`self.SaltoFin`))
  ; Movimiento Parabola
  (set `self.SaltoInicio` Inicio)
  (set `self.SaltoFin` (`KismetMathLibrary.MakeVector` (.x Destino) (.y Destino) (.z Inicio)))
  (bind (_direction _alpha) (`Timeline|Timeline` :!via `PlayFromStart`)
    (:`Update`
      (`self.K2_SetActorLocation` (+ (`KismetMathLibrary.VLerp` (`self.SaltoInicio`) _saltofin _alpha) (`KismetMathLibrary.MakeVector` 0.0 0.0 (* (* _alpha (- 1.0 _alpha)) (* (`self.AlturaSalto`) 4.0))))))
    (:`Finished`
      (`self.K2_SetActorLocation` _saltofin))))

(event `StartCracks`
  ; Cracks
  (bind _returnvalue (`KismetMaterialLibrary.CreateDynamicMaterialInstance` "/Game/Media/Visual/FX/Cracks/M_Cracks_Overlay_Inst.M_Cracks_Overlay_Inst"))
  (`MeshComponent.SetOverlayMaterial` (`self.ModelMesh`) _returnvalue)
  (`KismetSystemLibrary.DelayUntilNextTick`)
  (`AbilityAsync_WaitAttributeChanged.WaitForAttributeChanged` null (struct :`AttributeName` "Health" :`Attribute` "/Script/EgnisDef.HealthAttributeSet:Health" :`AttributeOwner` "/Script/CoreUObject.Class'/Script/EgnisDef.HealthAttributeSet'")
    (:`then`
      (`AbilityAsync_WaitAttributeChanged.WaitForAttributeChanged` null (struct :`AttributeName` "MaxHealth" :`Attribute` "/Script/EgnisDef.HealthAttributeSet:MaxHealth" :`AttributeOwner` "/Script/CoreUObject.Class'/Script/EgnisDef.HealthAttributeSet'")
        (:`then`
          _)
        (:`Changed`
          _)))
    (:`Changed`
      _))
  (`self.CracksRefresh`))

(event `CracksRefresh`
  ; Cracks
)

(event `self.ReceiveTick`
  (params (DeltaSeconds :type "Float (single-precision)"))
  ; Cracks
  (if (not (`EgnisAbilityLibrary.HasRule` self (struct :`TagName` "Rule.UI.HiddenHealth")))
    (bind _asmaterial_instance_dynamic (cast `MaterialInstanceDynamic` (`MeshComponent.GetOverlayMaterial` (`self.ModelMesh`))))
    (`MaterialInstanceDynamic.SetScalarParameterValue` _asmaterial_instance_dynamic "CrackAmount" (`KismetMathLibrary.MapRangeClamped` (`KismetMathLibrary.SafeDivide` (`self.GetCurrentHealth`) (`self.GetMaxHealth`)) 1.0 0.0 0.0 1.0))))

(event `SetSupportMark`
  (params (HealOn :type Boolean) (ShieldOn :type Boolean))
  (`SceneComponent.SetVisibility` (`self.HealMark`) HealOn false)
  (`SceneComponent.SetVisibility` (`self.ShieldMark`) ShieldOn false))

(event `EscucharDano`
  ;[0.9 0.9 0.9] Destello de dano: cada vez que baja la vida (atributo Health de GAS) se lanza el destello
  (bind (_asynctaskproxy _attribute _newvalue _oldvalue) (`AbilityAsync_WaitAttributeChanged.WaitForAttributeChanged` self (struct :`AttributeName` "Health" :`Attribute` "/Script/EgnisDef.HealthAttributeSet:Health" :`AttributeOwner` "/Script/CoreUObject.Class'/Script/EgnisDef.HealthAttributeSet'"))
    (:`then`
      ;[0.9 0.9 0.9] Tambien hay destello si el golpe se lo come el escudo (los aliados empiezan con InitialShield): asi siempre se ve que han recibido un golpe
      (bind (_asynctaskproxy_2 _attribute_2 _newvalue_2 _oldvalue_2) (`AbilityAsync_WaitAttributeChanged.WaitForAttributeChanged` self (struct :`AttributeName` "Shield" :`Attribute` "/Script/EgnisDef.HealthAttributeSet:Shield" :`AttributeOwner` "/Script/CoreUObject.Class'/Script/EgnisDef.HealthAttributeSet'"))
        (:`Changed`
          (if (< _newvalue_2 _oldvalue_2)
            (`self.MostrarDestelloDano`)))))
    (:`Changed`
      (if (< _newvalue _oldvalue)
        (`self.MostrarDestelloDano`)))))

(event `MostrarDestelloDano`
  ;[0.9 0.9 0.9] Poner el modelo en blanco y volver al material original pasados DuracionDestello segundos (si llega otro golpe, el tiempo se reinicia)
  (`self.PonerMaterialDestello`)
  ; Movimiento Parabola
  (`KismetSystemLibrary.RetriggerableDelay` (`self.DuracionDestello`))
  (`self.RestaurarMateriales`))

(fn `LanzarOnda`
  (params (Posicion :type "Vector Structure"))
  (`KismetMaterialLibrary.SetVectorParameterValue` "/Game/Media/Visual/Prototype/Materials/MPC_Onda.MPC_Onda" "OndaCentro" (make `LinearColor` (.x Posicion) (.y Posicion) (.z Posicion) 1.0))
  (`KismetMaterialLibrary.SetScalarParameterValue` "/Game/Media/Visual/Prototype/Materials/MPC_Onda.MPC_Onda" "OndaInicio" (`KismetSystemLibrary.GetGameTimeInSeconds`)))

(fn `ObtenerAlcance`
  (returns (Casillas :type "Array of TileCoord Structure"))
  (bind _outtiles (`GridMovementComponent.getRachableTiles` (`self.MoveComp`)))
  (return _outtiles))

(fn `PonerMaterialDestello`
  (bind _modelmesh (`self.ModelMesh`))
  ;[0.25 0.45 0.9] 1. Si no esta ya en blanco: guardar los materiales del modelo para restaurarlos despues
  (if (not (`self.bEnDestello`))
    (bind _output_get (set `self.MaterialesOriginales` (`MeshComponent.GetMaterials` _modelmesh)))
    (set `self.bEnDestello` true)
    ;[0.9 0.9 0.9] 2. Poner el material de destello (blanco) en todos los slots del modelo
    (for (_ _array_index) _output_get
      (`PrimitiveComponent.SetMaterial` _modelmesh _array_index (`self.MaterialDestello`)))))

(fn `PuedeIrA`
  (params (Casilla :type "TileCoord Structure"))
  (returns (Resultado :type Boolean))
  (bind _returnvalue (`GridMovementComponent.canMoveToTile` (`self.MoveComp`) Casilla))
  (return _returnvalue))

(fn `RestaurarMateriales`
  ;[0.9 0.9 0.9] Devolver a cada slot del modelo su material original y marcar que el destello ha terminado
  (for (_array_element _array_index) (`self.MaterialesOriginales`)
    (`PrimitiveComponent.SetMaterial` (`self.ModelMesh`) _array_index _array_element))
  (set `self.bEnDestello` false))

(fn `SetOutline`
  (params (Activo :type Boolean))
  (bind _ns_smokeaura (`self.NS_SmokeAura`))
  (if Activo
    (`ActorComponent.Activate` _ns_smokeaura true)
    (else
      (`ActorComponent.Deactivate` _ns_smokeaura))))

(fn `UserConstructionScript`)