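; GA_Jhunn is a unique gameplay ability for the ally Jhunn that turns Spirit Attraction into Burn on its owner.
; On activation it binds to the owner's status component and reacts whenever statuses change.
; If Spirit Attraction is present, it removes that status and applies Burn for a configurable number of turns, crediting the attraction's original source.
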(event `self.K2_ActivateAbility`
  (add `StatusEffectComponent.OnStatusChanged` (`CharacterBase.StatusComp` (`self.GetOwnerCharacter`)) (delegate `HandleStatusChanged`)))

(event `HandleStatusChanged`
  (bind _statuscomp (`CharacterBase.StatusComp` (`self.GetOwnerCharacter`)))
  (if (`StatusEffectComponent.HasStatus` _statuscomp "Status_SpiritAttraction")
    (set `self.Attractor` (`StatusEffectComponent.GetStatusSource` _statuscomp "Status_SpiritAttraction"))
    (`StatusEffectComponent.RemoveStatus` _statuscomp "Status_SpiritAttraction")
    (`StatusEffectComponent.ApplyStatus` _statuscomp "Status_Burn" (`self.BurnTurns`) (`self.Attractor`) "Default")))