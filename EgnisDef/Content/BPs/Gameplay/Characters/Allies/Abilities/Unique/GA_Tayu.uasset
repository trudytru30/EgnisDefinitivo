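; Tayu's unique ally ability, which spreads dealt damage to the enemies beside the target.
; It listens for Damage.Dealt events, acting when the card in play targets Enemy or no card is in play.
; HitRow plays an ivy effect through the owner, target and neighbors, then deals the same amount to each neighbor.
; An ApplyingRow flag stops that splash damage from re-triggering the ability.
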(event `self.K2_ActivateAbility`
  (bind _returnvalue (`EgnisAbilityLibrary.GetCardInPlay`))
  (bind (_asynctaskproxy _payload) (`AbilityTask_WaitGameplayEvent.WaitGameplayEvent` (struct :`TagName` "Event.Damage.Dealt") null)
    (:`EventReceived`
      (if (not (`self.ApplyingRow`))
        (bind ((`Target` _target) (`EventMagnitude` _eventmagnitude)) (break `GameplayEventData` _payload))
        (bind _ascharacter_base (cast `CharacterBase` _target))
        (if (`KismetSystemLibrary.IsValid` _returnvalue)
          (if (`|EnumEquality` (`BaseCard.GetTarget` _returnvalue) "Enemy")
            (`self.HitRow` _ascharacter_base _eventmagnitude :!label _label))
          (else
            (goto _label)))))))

(fn `HitRow`
  (params (RowTarget :type "CharacterBase Object Reference") (Amount :type "Float (double-precision)"))
  (bind _returnvalue (`self.GetOwnerCharacter`))
  (set `self.ApplyingRow` true)
  (`KismetArrayLibrary.Array_Clear` (`self.IvyPieces`))
  (`KismetArrayLibrary.Array_Add` (`self.IvyPieces`) _returnvalue)
  (`KismetArrayLibrary.Array_Add` (`self.IvyPieces`) RowTarget)
  (bind _returnvalue_2 (`EgnisAbilityLibrary.GetEnemiesBesideTarget` _returnvalue RowTarget))
  (for _array_element _returnvalue_2
    (`KismetArrayLibrary.Array_Add` (`self.IvyPieces`) _array_element))
  (`Card_IvyVFXEffect.PlayIvyThroughPieces` _returnvalue (`self.IvySettings`) (`self.IvyPieces`))
  (for _array_element_2 _returnvalue_2
    (`EgnisAbilityLibrary.DealDamage` _returnvalue _array_element_2 (`self.DamageEffect`) Amount))
  (set `self.ApplyingRow` false))