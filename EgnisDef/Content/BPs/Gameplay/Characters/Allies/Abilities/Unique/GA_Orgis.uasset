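; GA_Orgis is a unique ally gameplay ability that returns the previously played Cult.Egnis card from discard to hand on the first Egnis play each turn.
; It listens for turn-start events to reset the once-per-turn flag, and card-played events to check the instigator tags.
; Every Egnis play then becomes the stored last card.
; The first play spends the flag even when no valid card is stored.
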(event `self.K2_ActivateAbility`
  (bind _returnvalue (`EgnisAbilityLibrary.GetDeckManager`))
  (bind _lastegniscard (`self.LastEgnisCard`))
  (`|ExecutionSequence`
    (:`then_0`
      (`AbilityTask_WaitGameplayEvent.WaitGameplayEvent` (struct :`TagName` "Event.Turn.Start") null
        (:`EventReceived`
          (set `self.UsedEgnisThisTurn` false))))
    (:`then_1`
      (bind (_asynctaskproxy _payload) (`AbilityTask_WaitGameplayEvent.WaitGameplayEvent` (struct :`TagName` "Event.Card.Played") null)
        (:`EventReceived`
          (bind ((`OptionalObject` _optionalobject) (`InstigatorTags` _instigatortags)) (break `GameplayEventData` _payload))
          (if (`BlueprintGameplayTagLibrary.HasTag` _instigatortags (struct :`TagName` "Cult.Egnis") true)
            (if (not (`self.UsedEgnisThisTurn`))
              (set `self.UsedEgnisThisTurn` true)
              (if (and (`KismetSystemLibrary.IsValid` _returnvalue) (`KismetSystemLibrary.IsValid` _lastegniscard))
                (`DeckManager.ReturnCardFromDiscardToHand` _returnvalue _lastegniscard)))
            (set `self.LastEgnisCard` (cast `BaseCard` _optionalobject :!pure true))))))))