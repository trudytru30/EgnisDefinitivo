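; GA_Atanis is a unique ally gameplay ability that rewards unit deaths with minion cards at the start of the next turn.
; On activation it listens for unit death events and increments a pending card count for each one.
; When a turn start event arrives, it adds that many copies of MinionCard to the hand through the deck manager, then resets the count.
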(event `self.K2_ActivateAbility`
  (bind _returnvalue (`EgnisAbilityLibrary.GetDeckManager`))
  (bind _minioncard (`self.MinionCard`))
  (`|ExecutionSequence`
    (:`then_0`
      (`AbilityTask_WaitGameplayEvent.WaitGameplayEvent` (struct :`TagName` "Event.Unit.Died") null
        (:`EventReceived`
          (set `self.PendingCards` (+ (`self.PendingCards`) 1)))))
    (:`then_1`
      (`AbilityTask_WaitGameplayEvent.WaitGameplayEvent` (struct :`TagName` "Event.Turn.Start") null
        (:`EventReceived`
          (if (and (`KismetSystemLibrary.IsValid` _returnvalue) (`KismetSystemLibrary.IsValid` _minioncard))
            (for _ (range 1 (+ (`self.PendingCards`) 1))
              (`DeckManager.AddCardToHand` _returnvalue _minioncard)))
          (set `self.PendingCards` 0))))))