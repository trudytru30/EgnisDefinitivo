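; Ruinous Birth is an ally class Gameplay Ability that gives obstacles a limited lifetime and spawns spirit summons where they are destroyed.
; It listens for created-obstacle events to track turns left in a map, counting down each turn start and destroying expired obstacles.
; Destroyed-obstacle events queue the tile, and a next-tick timer spawns the owner's spirits there, with health scaled by Piety.
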(event `self.K2_ActivateAbility`
  (`|ExecutionSequence`
    (:`then_0`
      (bind (_asynctaskproxy _payload) (`AbilityTask_WaitGameplayEvent.WaitGameplayEvent` (struct :`TagName` "Event.Obstacle.Created") null)
        (:`EventReceived`
          (bind _asobstacle_base (cast `ObstacleBase` (`.Target` (break `GameplayEventData` _payload))))
          (`BlueprintMapLibrary.Map_Add` (`self.TurnsLeft`) _asobstacle_base (`self.LifetimeTurns`)))))
    (:`then_1`
      (`AbilityTask_WaitGameplayEvent.WaitGameplayEvent` (struct :`TagName` "Event.Turn.Start") null
        (:`EventReceived`
          (bind _keys (`BlueprintMapLibrary.Map_Keys` (`self.TurnsLeft`)))
          (for _array_element _keys
            (if (`KismetSystemLibrary.IsValid` _array_element)
              (bind _value (`BlueprintMapLibrary.Map_Find` (`self.TurnsLeft`) _array_element))
              (if (<= _value 1)
                (`ObstacleBase.HandleDestroyed` _array_element)
                (else
                  (`BlueprintMapLibrary.Map_Add` (`self.TurnsLeft`) _array_element (- _value 1))))
              (else
                (`BlueprintMapLibrary.Map_Remove` (`self.TurnsLeft`) _array_element)))))))
    (:`then_2`
      (bind (_asynctaskproxy_2 _payload_2) (`AbilityTask_WaitGameplayEvent.WaitGameplayEvent` (struct :`TagName` "Event.Obstacle.Destroyed") null)
        (:`EventReceived`
          (bind _asobstacle_base_2 (cast `ObstacleBase` (`.Target` (break `GameplayEventData` _payload_2))))
          (`BlueprintMapLibrary.Map_Remove` (`self.TurnsLeft`) _asobstacle_base_2)
          (`KismetArrayLibrary.Array_Add` (`self.PendingSpiritTiles`) (`ObstacleBase.CurrentTile` _asobstacle_base_2))
          (`KismetSystemLibrary.K2_SetTimerForNextTickDelegate` (delegate `SpawnPendingSpirits`)))))))

(event `SpawnPendingSpirits`
  (bind _returnvalue (`self.GetOwnerAlly`))
  (bind _pendingspirittiles (`self.PendingSpiritTiles`))
  (for _array_element _pendingspirittiles
    (`EgnisAbilityLibrary.SpawnSummon` _returnvalue (`self.SpiritClass`) (`self.SpiritData`) _array_element (* (`Ally.GetCharacterPiety` _returnvalue) (`self.SpiritPietyMultiplier`))))
  (`KismetArrayLibrary.Array_Clear` _pendingspirittiles))