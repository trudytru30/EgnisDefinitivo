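; Class gameplay ability Scarred Skin: the owner takes no Burn damage and turns its own Burn into an offensive tool.
; Whenever the owner's Burn turns rise, it re-applies Burn with twice the current turns, caching that count before applying to guard against re-triggering.
; A damage-dealt event listener applies Burn to enemy targets while the owner is burning and a card is in play.
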(event `self.K2_ActivateAbility`
  (bind _returnvalue (`self.GetOwnerCharacter`))
  (bind _statuscomp (`CharacterBase.StatusComp` _returnvalue))
  (`|ExecutionSequence`
    (:`then_0`
      (`EgnisAbilityLibrary.SetBurnDamageTaken` _returnvalue)
      (add `StatusEffectComponent.OnStatusChanged` _statuscomp (delegate `HandleStatusChanged`)))
    (:`then_1`
      (bind (_asynctaskproxy _payload) (`AbilityTask_WaitGameplayEvent.WaitGameplayEvent` (struct :`TagName` "Event.Damage.Dealt") null)
        (:`EventReceived`
          (bind ((`Target` _target)) (break `GameplayEventData` _payload))
          (if (and (and (`StatusEffectComponent.HasStatus` _statuscomp "Status_Burn") (`KismetSystemLibrary.IsValid` (`EgnisAbilityLibrary.GetCardInPlay`))) (`EgnisAbilityLibrary.AreEnemies` _returnvalue _target))
            (bind _ascharacter_base (cast `CharacterBase` _target))
            (`StatusEffectComponent.ApplyStatus` (`CharacterBase.StatusComp` _ascharacter_base) "Status_Burn" (`self.HitBurnTurns`) _returnvalue "Default")))))))

(event `HandleStatusChanged`
  (bind _statuscomp (`CharacterBase.StatusComp` (`self.GetOwnerCharacter`)))
  (bind _returnvalue (`StatusEffectComponent.GetTurnsLeft` _statuscomp "Status_Burn"))
  (if (> _returnvalue (`self.LastBurnTurns`))
    (set `self.LastBurnTurns` (* _returnvalue 2))
    (`StatusEffectComponent.ApplyStatus` _statuscomp "Status_Burn" (`self.LastBurnTurns`) (`StatusEffectComponent.GetStatusSource` _statuscomp "Status_Burn") "Default")
    (else
      (set `self.LastBurnTurns` _returnvalue))))