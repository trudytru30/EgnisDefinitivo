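; Gameplay ability for allied characters that makes slain enemies explode on the board, damaging and weakening other enemies nearby.
; On activation it waits for unit-killed gameplay events and filters for victims hostile to the owner.
; Explode gathers characters within a tile radius of the victim and deals enemies damage scaled from the owner's attack power.
; Targets still valid after the hit receive the Weakened status for a set number of turns.
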(event `self.K2_ActivateAbility`
  (bind (_asynctaskproxy _payload) (`AbilityTask_WaitGameplayEvent.WaitGameplayEvent` (struct :`TagName` "Event.Unit.Killed") null)
    (:`EventReceived`
      (bind _ascharacter_base (cast `CharacterBase` (`.Target` (break `GameplayEventData` _payload))))
      (if (`EgnisAbilityLibrary.AreEnemies` (`self.GetOwnerCharacter`) _ascharacter_base)
        (`self.Explode` _ascharacter_base)))))

(fn `Explode`
  (params (Center :type "CharacterBase Object Reference"))
  (bind _returnvalue (`self.GetOwnerCharacter`))
  (bind _returnvalue_2 (`EgnisAbilityLibrary.GetCharactersAround` (`CharacterBase.Board` _returnvalue) (`CharacterBase.CurrentTile` Center) (`self.Radius`)))
  (for _array_element _returnvalue_2
    (if (`EgnisAbilityLibrary.AreEnemies` _returnvalue _array_element)
      (`EgnisAbilityLibrary.DealDamage` _returnvalue _array_element (`self.DamageEffect`) (`EgnisCombatLibrary.CalculateDamage` _returnvalue _array_element (* (`EgnisCombatLibrary.GetAttackPower` _returnvalue) (`self.DamageMultiplier`))))
      (if (`KismetSystemLibrary.IsValid` _array_element)
        (`StatusEffectComponent.ApplyStatus` (`CharacterBase.StatusComp` _array_element) "Status_Weakened" (`self.WeakenedTurns`) _returnvalue)))))