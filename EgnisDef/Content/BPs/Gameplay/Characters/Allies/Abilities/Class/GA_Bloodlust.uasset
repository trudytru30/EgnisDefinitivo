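; GA_Bloodlust is a class ability for allies that builds and clears Bloodlust stacks in a card-based, turn-based game.
; It listens for gameplay events in parallel: the first Wers cult card played each turn adds one stack.
; Turn end clears all stacks if that flag is unset, then resets it.
; Fury consume clears stacks and sets the flag, while max Fury applies stacks up to the limit.
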(event `self.K2_ActivateAbility`
  (`|ExecutionSequence`
    (:`then_0`
      (bind (_asynctaskproxy _payload) (`AbilityTask_WaitGameplayEvent.WaitGameplayEvent` (struct :`TagName` "Event.Card.Played") null)
        (:`EventReceived`
          (if (`BlueprintGameplayTagLibrary.HasTag` (`.InstigatorTags` (break `GameplayEventData` _payload)) (struct :`TagName` "Cult.Wers") true)
            (if (not (`self.bUsedWersThisTurn`))
              (set `self.bUsedWersThisTurn` true)
              (`self.BP_ApplyGameplayEffectToOwner` "/Game/BPs/Gameplay/Characters/Allies/Abilities/Class/Effects/BP_BloodlustEffect.BP_BloodlustEffect_C"))))))
    (:`then_1`
      (`AbilityTask_WaitGameplayEvent.WaitGameplayEvent` (struct :`TagName` "Event.Turn.End") null
        (:`then`
          (`AbilityTask_WaitGameplayEvent.WaitGameplayEvent` (struct :`TagName` "Event.Fury.Consume") null
            (:`then`
              (`AbilityTask_WaitGameplayEvent.WaitGameplayEvent` (struct :`TagName` "Event.Fury.Max") null
                (:`EventReceived`
                  (`self.BP_ApplyGameplayEffectToOwner` "/Game/BPs/Gameplay/Characters/Allies/Abilities/Class/Effects/BP_BloodlustEffect.BP_BloodlustEffect_C" 1 (`EgnisAbilityLibrary.GetEffectStackLimit` "/Game/BPs/Gameplay/Characters/Allies/Abilities/Class/Effects/BP_BloodlustEffect.BP_BloodlustEffect_C")))))
            (:`EventReceived`
              (`AbilitySystemComponent.RemoveActiveGameplayEffectBySourceEffect` (`self.GetAbilitySystemComponentFromActorInfo`) "/Game/BPs/Gameplay/Characters/Allies/Abilities/Class/Effects/BP_BloodlustEffect.BP_BloodlustEffect_C" null -1)
              (set `self.bUsedWersThisTurn` true))))
        (:`EventReceived`
          (if (not (`self.bUsedWersThisTurn`))
            (`AbilitySystemComponent.RemoveActiveGameplayEffectBySourceEffect` (`self.GetAbilitySystemComponentFromActorInfo`) "/Game/BPs/Gameplay/Characters/Allies/Abilities/Class/Effects/BP_BloodlustEffect.BP_BloodlustEffect_C" null -1))
          (set `self.bUsedWersThisTurn` false))))))