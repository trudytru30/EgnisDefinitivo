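; GA_Seeding is a gameplay ability that plays an ivy visual linking its owner to seeding targets when cards are used.
; It listens for damage-dealt and card-played events, showing ivy early on damage from an enemy-targeted card, otherwise when an ally- or enemy-targeted card is played.
; The IvyShown flag prevents a repeat and resets after each card-played event.
; ShowIvy gathers targets on the relevant side and runs ivy through them.
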(event `self.K2_ActivateAbility`
  (bind _returnvalue (`EgnisAbilityLibrary.GetCardInPlay`))
  (`|ExecutionSequence`
    (:`then_0`
      (`AbilityTask_WaitGameplayEvent.WaitGameplayEvent` (struct :`TagName` "Event.Damage.Dealt") null
        (:`EventReceived`
          (if (`KismetSystemLibrary.IsValid` _returnvalue)
            (if (and (`|EnumEquality` (`BaseCard.GetTarget` _returnvalue) "Enemy") (not (`self.IvyShown`)))
              (set `self.IvyShown` true)
              (`self.ShowIvy` false))))))
    (:`then_1`
      (bind (_asynctaskproxy _payload) (`AbilityTask_WaitGameplayEvent.WaitGameplayEvent` (struct :`TagName` "Event.Card.Played") null)
        (:`EventReceived`
          (bind _asbase_card (cast `BaseCard` (`.OptionalObject` (break `GameplayEventData` _payload)))
            (:`then`
              (if (not (`self.IvyShown`))
                (bind _returnvalue_2 (`BaseCard.GetTarget` _asbase_card))
                (bind _returnvalue_3 (`|EnumEquality` _returnvalue_2 "Ally"))
                (if (or _returnvalue_3 (`|EnumEquality` _returnvalue_2 "Enemy"))
                  (`self.ShowIvy` _returnvalue_3))))
            (:`CastFailed`
              _))
          (set `self.IvyShown` false))))))

(fn `ShowIvy`
  (params (bAllies :type Boolean))
  (bind _returnvalue (`self.GetOwnerCharacter`))
  (`KismetArrayLibrary.Array_Clear` (`self.IvyPieces`))
  (`KismetArrayLibrary.Array_Add` (`self.IvyPieces`) _returnvalue)
  (bind _returnvalue_2 (`EgnisAbilityLibrary.GetSeedingTargets` _returnvalue bAllies))
  (for _array_element _returnvalue_2
    (`KismetArrayLibrary.Array_Add` (`self.IvyPieces`) _array_element))
  (if (> (`KismetArrayLibrary.Array_Length` (`self.IvyPieces`)) 1)
    (`Card_IvyVFXEffect.PlayIvyThroughPieces` _returnvalue (`self.IvySettings`) (`self.IvyPieces`))))