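; Moon Mantle is an ally class gameplay ability that shields non-enemy characters around its owner when a turn ends without movement.
; It listens for turn start, unit moved and turn end gameplay events, using the first two to reset and set a moved flag.
; At turn end it queries board characters within a radius, grants each non-enemy a shield effect, and plays one sound if any was shielded.
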(event `self.K2_ActivateAbility`
  (bind _returnvalue (`self.GetOwnerCharacter`))
  (`|ExecutionSequence`
    (:`then_0`
      (`AbilityTask_WaitGameplayEvent.WaitGameplayEvent` (struct :`TagName` "Event.Turn.Start") null
        (:`EventReceived`
          (set `self.MovedThisTurn` false))))
    (:`then_1`
      (`AbilityTask_WaitGameplayEvent.WaitGameplayEvent` (struct :`TagName` "Event.Unit.Moved") null
        (:`EventReceived`
          (set `self.MovedThisTurn` true))))
    (:`then_2`
      (`AbilityTask_WaitGameplayEvent.WaitGameplayEvent` (struct :`TagName` "Event.Turn.End") null
        (:`EventReceived`
          (if (not (`self.MovedThisTurn`))
            (set `self.Shielded` false)
            (bind _returnvalue_2 (`EgnisAbilityLibrary.GetCharactersAround` (`CharacterBase.Board` _returnvalue) (`CharacterBase.CurrentTile` _returnvalue) (`self.Radius`)))
            (for _array_element _returnvalue_2
              (if (not (`EgnisAbilityLibrary.AreEnemies` _returnvalue _array_element))
                (`EgnisAbilityLibrary.GrantShield` _returnvalue _array_element (`self.ShieldEffect`) (`self.ShieldAmount`))
                (set `self.Shielded` true)))
            (if (`self.Shielded`)
              (`AudioManager.PlayTrigger` (subsystem `AudioManager`) "CardShield" null _returnvalue))))))))