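; Player controller for the tactical card board game, handling ally selection, piece movement and card-targeting feedback.
; Right-click lifts a piece to drag, or on its own tile enters click-to-move; RequestUnitMove validates before the jump.
; Tick updates enemy highlight, attack and support marks, plus range, area and push/pull previews for the pending card.
; A Niagara wisp (FuegoFatuo) trails the cursor while active with a pending card.
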(event Input|EnhancedActionEvents|EnhancedInputActionIA_RightClick
  (params (ActionValue :type Boolean) (ElapsedSeconds :type Float%20%28double-precision%29) (TriggeredSeconds :type Float%20%28double-precision%29) (InputAction :type Input%20Action%20Object%20Reference :default "/Game/Inputs/IA_RightClick.IA_RightClick"))
  (bind (_hitresult _returnvalue) (Game|Player|GetHitResultUnderCursorbyChannel "TraceTypeQuery4" true))
  (bind (_hitresult_2 _returnvalue_2) (Game|Player|GetHitResultUnderCursorbyChannel "TraceTypeQuery4" true))
  ;[0.15 0.15 0.15 0.5] Preview Mov
  (:Triggered
    (if (Utilities|IsValid (Variables|Default|GetPiezaArrastrada))
      (if (and _returnvalue (.ReturnValue (Class|Board|WorldPointtoTile (Variables|/Script/EgnisDef.CharacterBase|GetBoard (Variables|Default|GetPiezaArrastrada)) (.ImpactPoint (Collision|BreakHitResult _hitresult)))))
        (bind _resultado (Default|PuedeIrA (Variables|Default|GetPiezaArrastrada) (.OutTile (Class|Board|WorldPointtoTile (Variables|/Script/EgnisDef.CharacterBase|GetBoard (Variables|Default|GetPiezaArrastrada)) (.ImpactPoint (Collision|BreakHitResult _hitresult))))))
        (Default|MostrarMarcador (.AsBP%20Board (Utilities|Casting|CastToBP_Board (Variables|/Script/EgnisDef.CharacterBase|GetBoard (Variables|Default|GetPiezaArrastrada)))) (.OutTile (Class|Board|WorldPointtoTile (Variables|/Script/EgnisDef.CharacterBase|GetBoard (Variables|Default|GetPiezaArrastrada)) (.ImpactPoint (Collision|BreakHitResult _hitresult)))) _resultado)
        (else
          (Default|OcultarMarcador (.AsBP%20Board (Utilities|Casting|CastToBP_Board (Variables|/Script/EgnisDef.CharacterBase|GetBoard (Variables|Default|GetPiezaArrastrada)))))))))
  (:Started
    (bind _asbp_ally (Utilities|Casting|CastToBP_Ally (.HitActor (Collision|BreakHitResult (.HitResult (Game|Player|GetHitResultUnderCursorbyChannel "TraceTypeQuery3" true)))))
      (:then
        (if (Class|BoardPlayerController|CanUnitMoveThisTurn _asbp_ally)
          (Class|BoardPlayerController|SelectDraggedAlly _asbp_ally)
          (bind _output_get (Variables|Default|SetPiezaArrastrada _asbp_ally))
          (bind _output_get_2 (Variables|Default|SetPosInicial (Transformation|GetActorLocation _output_get)))
          (Transformation|SetActorLocation _output_get (+ _output_get_2 "0.000000,0.000000,25.000000") false false)
          (bind _casillas (Default|ObtenerAlcance _output_get))
          (Default|MostrarAlcance (.AsBP%20Board (Utilities|Casting|CastToBP_Board (Variables|/Script/EgnisDef.CharacterBase|GetBoard (Variables|Default|GetPiezaArrastrada)))) _casillas)
          (Class|CharacterBase|PlayPieceLiftSound _asbp_ally)))
      (:CastFailed
        (MovimientoClick|ClickMoverIntentarMover :!pinned true) ; MODO CLICK: click derecho fuera de un aliado = mover la pieza activa a esa casilla
      )))
  (:Completed
    (if (Utilities|IsValid (Variables|Default|GetPiezaArrastrada))
      (Default|OcultarMarcador (.AsBP%20Board (Utilities|Casting|CastToBP_Board (Variables|/Script/EgnisDef.CharacterBase|GetBoard (Variables|Default|GetPiezaArrastrada)))))
      (Default|OcultarAlcance (.AsBP%20Board (Utilities|Casting|CastToBP_Board (Variables|/Script/EgnisDef.CharacterBase|GetBoard (Variables|Default|GetPiezaArrastrada)))))
      (MovimientoClick|ClickMoverAlSoltar :!pinned true) ; MODO CLICK: soltar sobre la propia casilla = activar / cancelar
      (if (and _returnvalue_2 (.ReturnValue (Class|Board|WorldPointtoTile (Variables|/Script/EgnisDef.CharacterBase|GetBoard (Variables|Default|GetPiezaArrastrada)) (.ImpactPoint (Collision|BreakHitResult _hitresult_2)))))
        (bind _returnvalue_3 (Class|BoardPlayerController|RequestUnitMove (Variables|Default|GetPiezaArrastrada) (.OutTile (Class|Board|WorldPointtoTile (Variables|/Script/EgnisDef.CharacterBase|GetBoard (Variables|Default|GetPiezaArrastrada)) (.ImpactPoint (Collision|BreakHitResult _hitresult_2))))))
        (if _returnvalue_3
          (Default|SaltarA (Variables|Default|GetPiezaArrastrada) (Variables|Default|GetPosInicial) (Class|CharacterBase|GetStandLocationforTile (Variables|Default|GetPiezaArrastrada) (.OutTile (Class|Board|WorldPointtoTile (Variables|/Script/EgnisDef.CharacterBase|GetBoard (Variables|Default|GetPiezaArrastrada)) (.ImpactPoint (Collision|BreakHitResult _hitresult_2))))))
          (elif (Utilities|IsValid (Variables|Default|GetPiezaArrastrada))
            (Transformation|SetActorLocation (Variables|Default|GetPiezaArrastrada) (Variables|Default|GetPosInicial) false false :!label _label)))
        (else
          (goto _label)))
      (Variables|Default|SetPiezaArrastrada 0))))

(event Input|EnhancedActionEvents|EnhancedInputActionIA_LeftClick
  (params (ActionValue :type Boolean) (ElapsedSeconds :type Float%20%28double-precision%29) (TriggeredSeconds :type Float%20%28double-precision%29) (InputAction :type Input%20Action%20Object%20Reference :default "/Game/Inputs/IA_LeftClick.IA_LeftClick"))
  ;[0.15 0.15 0.15 0.5] Outline Pieza
  (:Started
    (bind _asbp_ally (Utilities|Casting|CastToBP_Ally (.HitActor (Collision|BreakHitResult (.HitResult (Game|Player|GetHitResultUnderCursorbyChannel "TraceTypeQuery3" true))))))
    (if (Utilities|IsValid (Variables|Default|GetPiezaSeleccionada))
      (Default|SetOutline (Variables|Default|GetPiezaSeleccionada) false))
    (bind _output_get (Variables|Default|SetPiezaSeleccionada _asbp_ally))
    (Default|SetOutline _output_get true)))

(event EventRefreshHandUI
  (bind _aswbp_game_hud (Utilities|Casting|CastToWBP_GameHUD (Variables|Default|GetHUD%20WIdget)))
  (Default|SetHand _aswbp_game_hud (Class|BoardPlayerController|GetCurrentHand)))

(event EventOnKeyboardAllySelected
  (params (Ally :type Character%20Base%20Object%20Reference))
  (bind _asbp_ally (Utilities|Casting|CastToBP_Ally Ally))
  (if (Utilities|IsValid (Variables|Default|GetPiezaSeleccionada))
    (Default|SetOutline (Variables|Default|GetPiezaSeleccionada) false))
  (Variables|Default|SetPiezaSeleccionada _asbp_ally)
  (Default|SetOutline _asbp_ally true))

(event EventTick
  (params (DeltaSeconds :type Float%20%28single-precision%29))
  ;[0.15 0.15 0.15 0.5] Mark
  (CallFunction|ActualizarEnemigoBajoCursor)
  (CallFunction|UpdateAttackMarks)
  (CallFunction|UpdateSupportMark)
  (CallFunction|ActualizarPreviewAtaque)
  (CallFunction|ActualizarFuegoFatuo))

(fn ConstructionScript)

(fn UpdateAttackMarks
  (bind _returnvalue (Class|BoardPlayerController|GetSelectedAlly))
  (bind _pendingcard (Variables|Default|GetPendingCard))
  (bind (_asally _bsuccess) (Utilities|Casting|CastToAlly _returnvalue))
  (bind _outactors (Actor|GetAllActorsOfClass "/Script/EgnisDef.Enemy"))
  (for _array_element _outactors
    (if (and _bsuccess (Utilities|IsValid (Variables|Default|GetPendingCard)))
      (Class|BPIAttackMark|SetAttackMark(Message) _array_element (Math|Boolean|ANDBoolean (Utilities|Enum|Equal(Enum) (Class|BaseCard|GetTarget _pendingcard) "Enemy") (Utilities|Enum|Equal(Enum) (Class|BaseCard|GetCardType _pendingcard) "Attack") (Class|Ally|CanPayCardCost _asally _pendingcard) (Class|EgnisCombatLibrary|CanAct _asally) (Class|BaseCard|CanbePlayedby _pendingcard _asally) (Utilities|Array|ContainsItem (Variables|PreviewAtaque|GetCasillasRangoAtaque) (Variables|/Script/EgnisDef.CharacterBase|GetCurrentTile _array_element))))
      (else
        (Class|BPIAttackMark|SetAttackMark(Message) _array_element false)))))

(fn UpdateSupportMark
  (bind _pendingcard (Variables|Default|GetPendingCard))
  (bind _pendingcard_2 (Variables|Default|GetPendingCard))
  (bind _returnvalue (Class|BaseCard|GetTarget _pendingcard_2))
  (Variables|Default|SetIsHeal false)
  (Variables|Default|SetIsShield false)
  (if (Utilities|IsValid _pendingcard)
    (for _array_element (Variables|/Script/EgnisDef.BaseCard|GetEffects _pendingcard)
      (Utilities|Casting|CastToCard_HealEffect _array_element
        (:then
          (Variables|Default|SetIsHeal true))
        (:CastFailed
          (Utilities|Casting|CastToCard_ShieldEffect _array_element)
          (Variables|Default|SetIsShield true)))))
  ;[0.1 0.15 0.3] 2. Para cada aliado: cast, lanzador y encender o apagar sus m
  (bind _outactors (Actor|GetAllActorsOfClass "/Game/BPs/Gameplay/Characters/Allies/BP_Ally.BP_Ally_C"))
  (for _array_element_2 _outactors
    (bind _asbp_ally (Utilities|Casting|CastToBP_Ally _array_element_2))
    (bind _asally (Utilities|Casting|CastToAlly (Class|BoardPlayerController|GetSelectedAlly))
      (:then
        (if (Utilities|IsValid _pendingcard_2)
          (Default|SetSupportMark _asbp_ally (and (and (and (Class|BaseCard|CanbePlayedby _pendingcard_2 _asally) (Class|Ally|CanPayCardCost _asally _pendingcard_2)) (and (Class|EgnisCombatLibrary|IsCardTargetinRange _pendingcard_2 _asally _asbp_ally (Math|Vector|MakeVector 0.0 0.0 0.0)) (or (Utilities|Enum|Equal(Enum) _returnvalue "Ally") (and (Utilities|Enum|Equal(Enum) _returnvalue "Self") (== _asbp_ally _asally))))) (Variables|Default|GetIsHeal)) (and (and (and (Class|BaseCard|CanbePlayedby _pendingcard_2 _asally) (Class|Ally|CanPayCardCost _asally _pendingcard_2)) (and (Class|EgnisCombatLibrary|IsCardTargetinRange _pendingcard_2 _asally _asbp_ally (Math|Vector|MakeVector 0.0 0.0 0.0)) (or (Utilities|Enum|Equal(Enum) _returnvalue "Ally") (and (Utilities|Enum|Equal(Enum) _returnvalue "Self") (== _asbp_ally _asally))))) (Variables|Default|GetIsShield)))
          (else
            (Default|SetSupportMark _asbp_ally false false :!label _label))))
      (:CastFailed
        (goto _label)))))

(fn ActualizarPreviewAtaque
  (Utilities|FlowControl|Sequence
    (:then_0
      (if (!= (Variables|Default|GetPendingCard) (Variables|PreviewAtaque|GetCartaPreview))
        (CallFunction|RefrescarRangoAtaque)))
    (:then_1
      (CallFunction|PreviewCursorAtaque))))

(fn RefrescarRangoAtaque
  (bind _returnvalue (Class|BoardPlayerController|GetSelectedAlly))
  (Variables|PreviewAtaque|SetCartaPreview (Variables|Default|GetPendingCard))
  (Variables|PreviewAtaque|SetRadioAreaPreview 0)
  (if (Utilities|IsValid (Variables|PreviewAtaque|GetBoardPreview))
    (Default|OcultarRangoAtaque (Variables|PreviewAtaque|GetBoardPreview))
    (Default|OcultarMarcador (Variables|PreviewAtaque|GetBoardPreview)))
  (if (Utilities|IsValid (Variables|PreviewAtaque|GetCartaPreview))
    (bind _returnvalue_2 (Actor|GetActorOfClass "/Game/BPs/Gameplay/Environment/Board/BP_Board.BP_Board_C"))
    (Variables|PreviewAtaque|SetBoardPreview _returnvalue_2)
    (if (and (Class|EgnisAbilityLibrary|HasRule _returnvalue "(TagName=\"Rule.Targeting.Seeding\")") (or (Utilities|Enum|Equal(Enum) (Class|BaseCard|GetTarget (Variables|PreviewAtaque|GetCartaPreview)) "Ally") (Utilities|Enum|Equal(Enum) (Class|BaseCard|GetTarget (Variables|PreviewAtaque|GetCartaPreview)) "Enemy")))
      (bind _returnvalue_3 (Class|EgnisAbilityLibrary|GetSeedingTargets _returnvalue (Utilities|Enum|Equal(Enum) (Class|BaseCard|GetTarget (Variables|PreviewAtaque|GetCartaPreview)) "Ally")))
      (Utilities|Array|Clear (Variables|PreviewAtaque|GetCasillasRangoAtaque))
      (for _array_element _returnvalue_3
        (Utilities|Array|Add (Variables|PreviewAtaque|GetCasillasRangoAtaque) (Variables|/Script/EgnisDef.CharacterBase|GetCurrentTile _array_element)))
      (else
        (Variables|PreviewAtaque|SetCasillasRangoAtaque (.OutTiles (Class|BoardPlayerController|GetPendingCardRangeTiles)))))
    (Default|MostrarRangoAtaque (Variables|PreviewAtaque|GetBoardPreview) (Variables|PreviewAtaque|GetCasillasRangoAtaque))
    (for _array_element_2 (Variables|/Script/EgnisDef.BaseCard|GetEffects (Variables|PreviewAtaque|GetCartaPreview))
      (bind _ascard_area_damage_effect (Utilities|Casting|CastToCard_AreaDamageEffect _array_element_2))
      (Variables|PreviewAtaque|SetRadioAreaPreview (Variables|/Script/EgnisDef.Card_AreaDamageEffect|GetAreaRadius _ascard_area_damage_effect)))))

(fn PreviewCursorAtaque
  (bind _cartapreview (Variables|PreviewAtaque|GetCartaPreview))
  (bind _boardpreview (Variables|PreviewAtaque|GetBoardPreview))
  (bind _radioareapreview (Variables|PreviewAtaque|GetRadioAreaPreview))
  (bind _returnvalue (Class|BaseCard|GetTarget _cartapreview))
  (bind _returnvalue_2 (Utilities|Enum|Equal(Enum) _returnvalue "Tile"))
  (if (and (and (Utilities|IsValid _cartapreview) (Utilities|IsValid _boardpreview)) (not (Utilities|IsValid (Variables|Default|GetPiezaArrastrada))))
    (bind _returnvalue_3 (Class|WidgetLayoutLibrary|GetMousePositiononPlatform))
    (bind (_outhit _returnvalue_4) (Collision|LineTraceByChannel (.WorldLocation (Class|PlayerController|DeprojectScreenPositiontoWorld (.X (Math|Vector2D|BreakVector2D (.PixelPosition (Class|SlateBlueprintLibrary|AbsolutetoViewport _returnvalue_3)))) (.Y (Math|Vector2D|BreakVector2D (.PixelPosition (Class|SlateBlueprintLibrary|AbsolutetoViewport _returnvalue_3)))))) (+ (.WorldLocation (Class|PlayerController|DeprojectScreenPositiontoWorld (.X (Math|Vector2D|BreakVector2D (.PixelPosition (Class|SlateBlueprintLibrary|AbsolutetoViewport _returnvalue_3)))) (.Y (Math|Vector2D|BreakVector2D (.PixelPosition (Class|SlateBlueprintLibrary|AbsolutetoViewport _returnvalue_3)))))) (* (.WorldDirection (Class|PlayerController|DeprojectScreenPositiontoWorld (.X (Math|Vector2D|BreakVector2D (.PixelPosition (Class|SlateBlueprintLibrary|AbsolutetoViewport _returnvalue_3)))) (.Y (Math|Vector2D|BreakVector2D (.PixelPosition (Class|SlateBlueprintLibrary|AbsolutetoViewport _returnvalue_3)))))) 2e+05)) "TraceTypeQuery4" true 0 "None"))
    (if (and _returnvalue_4 (.ReturnValue (Class|Board|WorldPointtoTile _boardpreview (.ImpactPoint (Collision|BreakHitResult _outhit)))))
      (bind _asally (Utilities|Casting|CastToAlly (Class|BoardPlayerController|GetSelectedAlly))
        (:then
          _)
        (:CastFailed
          _))
      (bind _valido (CallFunction|ObjetivoValidoEnCasilla (.OutTile (Class|Board|WorldPointtoTile _boardpreview (.ImpactPoint (Collision|BreakHitResult _outhit)))) (.ImpactPoint (Collision|BreakHitResult _outhit))))
      (Default|MostrarMarcador _boardpreview (.OutTile (Class|Board|WorldPointtoTile _boardpreview (.ImpactPoint (Collision|BreakHitResult _outhit)))) (or (and _returnvalue_2 (Class|EgnisCombatLibrary|IsCardTargetinRange _cartapreview _asally 0 (.ImpactPoint (Collision|BreakHitResult _outhit)))) (and (not _returnvalue_2) _valido)))
      (if (and (or (and _returnvalue_2 (Class|EgnisCombatLibrary|IsCardTargetinRange _cartapreview _asally 0 (.ImpactPoint (Collision|BreakHitResult _outhit)))) (and (not _returnvalue_2) _valido)) (> _radioareapreview 0))
        (Variables|PreviewAtaque|SetCasillasAreaPreview (Class|Board|GetTilesinRange _boardpreview (.OutTile (Class|Board|WorldPointtoTile _boardpreview (.ImpactPoint (Collision|BreakHitResult _outhit)))) _radioareapreview))
        (Utilities|Array|Add (Variables|PreviewAtaque|GetCasillasAreaPreview) (.OutTile (Class|Board|WorldPointtoTile _boardpreview (.ImpactPoint (Collision|BreakHitResult _outhit)))))
        (Default|MostrarArea _boardpreview (Variables|PreviewAtaque|GetCasillasAreaPreview))
        (elif (or (and _returnvalue_2 (Class|EgnisCombatLibrary|IsCardTargetinRange _cartapreview _asally 0 (.ImpactPoint (Collision|BreakHitResult _outhit)))) (and (not _returnvalue_2) _valido))
          (bind _casillas (CallFunction|CasillasEmpuje (.OutTile (Class|Board|WorldPointtoTile _boardpreview (.ImpactPoint (Collision|BreakHitResult _outhit))))))
          (Default|MostrarArea _boardpreview _casillas)
          (else
            (Default|MostrarArea _boardpreview))))
      (else
        (Default|OcultarMarcador _boardpreview)
        (Default|MostrarArea _boardpreview)))))

(fn PuedeLanzarCarta
  (params (Carta :type Base%20Card%20Object%20Reference))
  (bind _returnvalue (Class|BoardPlayerController|GetSelectedAlly))
  (bind _returnvalue_2 (Class|BaseCard|GetTarget Carta))
  (bind _returnvalue_3 (Utilities|Enum|Equal(Enum) _returnvalue_2 "Ally"))
  (bind _returnvalue_4 (Class|EgnisAbilityLibrary|GetSeedingTargets _returnvalue _returnvalue_3))
  (return (not (and (and (and (Class|EgnisAbilityLibrary|HasRule _returnvalue "(TagName=\"Rule.Targeting.Seeding\")") (or _returnvalue_3 (Utilities|Enum|Equal(Enum) _returnvalue_2 "Enemy"))) (== (Utilities|Array|Length _returnvalue_4) 0)) (not (Class|DeckManager|IsSelectingfromHand (Class|EgnisAbilityLibrary|GetDeckManager)))))))

(fn CasillasEmpuje
  (params (Casilla :type Tile%20Coord%20Structure))
  (bind (_x _y) (Utilities|Struct|BreakTileCoord Casilla))
  (bind _returnvalue (Class|BoardPlayerController|GetSelectedAlly))
  (bind _boardpreview (Variables|PreviewAtaque|GetBoardPreview))
  (bind _empujeresultado (Variables|PreviewEmpuje|GetEmpujeResultado))
  (bind _currenttile (Variables|/Script/EgnisDef.CharacterBase|GetCurrentTile _returnvalue))
  (bind (_x_2 _y_2) (Utilities|Struct|BreakTileCoord _currenttile))
  (bind _returnvalue_2 (- _x _x_2))
  (bind _returnvalue_3 (- _y _y_2))
  (bind _returnvalue_4 (Math|Integer|Absolute(Integer) _returnvalue_2))
  (bind _returnvalue_5 (Math|Integer|Absolute(Integer) _returnvalue_3))
  (Utilities|Array|Clear _empujeresultado)
  (if (Utilities|IsValid (Class|Board|GetTileOccupant _boardpreview Casilla))
    (for _array_element (Variables|/Script/EgnisDef.BaseCard|GetEffects (Variables|PreviewAtaque|GetCartaPreview))
      (bind _ascard_push_pull_effect (Utilities|Casting|CastToCard_PushPullEffect _array_element))
      (Variables|PreviewEmpuje|SetEmpujeDestino Casilla)
      (Variables|PreviewEmpuje|SetEmpujeBloqueado false)
      (Variables|PreviewEmpuje|SetEmpujeMovido false)
      (for _index (range 1 (Math|Integer|SelectInt (Math|Integer|Min(Integer) (Variables|/Script/EgnisDef.Card_PushPullEffect|GetDistance _ascard_push_pull_effect) (- (Math|Integer|Max(Integer) _returnvalue_4 _returnvalue_5) 1)) (Variables|/Script/EgnisDef.Card_PushPullEffect|GetDistance _ascard_push_pull_effect) (Utilities|Enum|Equal(Enum) (Variables|/Script/EgnisDef.Card_PushPullEffect|GetMode _ascard_push_pull_effect) "Pull")))
        (if (not (Variables|PreviewEmpuje|GetEmpujeBloqueado))
          (if (Class|Board|IsTileOccupied _boardpreview (Utilities|Struct|MakeTileCoord (+ _x (* (Math|Integer|SelectInt (* (Math|Integer|SelectInt -1 1 (Utilities|Enum|Equal(Enum) (Variables|/Script/EgnisDef.Card_PushPullEffect|GetMode _ascard_push_pull_effect) "Pull")) (Class|KismetMathLibrary|SignOfInteger _returnvalue_2)) 0 (>= _returnvalue_4 _returnvalue_5)) _index)) (+ _y (* (Math|Integer|SelectInt (* (Math|Integer|SelectInt -1 1 (Utilities|Enum|Equal(Enum) (Variables|/Script/EgnisDef.Card_PushPullEffect|GetMode _ascard_push_pull_effect) "Pull")) (Class|KismetMathLibrary|SignOfInteger _returnvalue_3)) 0 (>= _returnvalue_5 _returnvalue_4)) _index))))
            (Variables|PreviewEmpuje|SetEmpujeBloqueado true)
            (else
              (Variables|PreviewEmpuje|SetEmpujeDestino (Utilities|Struct|MakeTileCoord (+ _x (* (Math|Integer|SelectInt (* (Math|Integer|SelectInt -1 1 (Utilities|Enum|Equal(Enum) (Variables|/Script/EgnisDef.Card_PushPullEffect|GetMode _ascard_push_pull_effect) "Pull")) (Class|KismetMathLibrary|SignOfInteger _returnvalue_2)) 0 (>= _returnvalue_4 _returnvalue_5)) _index)) (+ _y (* (Math|Integer|SelectInt (* (Math|Integer|SelectInt -1 1 (Utilities|Enum|Equal(Enum) (Variables|/Script/EgnisDef.Card_PushPullEffect|GetMode _ascard_push_pull_effect) "Pull")) (Class|KismetMathLibrary|SignOfInteger _returnvalue_3)) 0 (>= _returnvalue_5 _returnvalue_4)) _index))))
              (Variables|PreviewEmpuje|SetEmpujeMovido true)))))
      (if (Variables|PreviewEmpuje|GetEmpujeMovido)
        (Utilities|Array|Add _empujeresultado (Variables|PreviewEmpuje|GetEmpujeDestino)))))
  (return _empujeresultado))

(fn ObjetivoValidoEnCasilla
  (params (Casilla :type Tile%20Coord%20Structure) (Punto :type Vector))
  (bind _cartapreview (Variables|PreviewAtaque|GetCartaPreview))
  (bind _returnvalue (Class|BaseCard|GetTarget _cartapreview))
  (bind _ascharacter_base (Utilities|Casting|CastToCharacterBase (Class|Board|GetTileOccupant (Variables|PreviewAtaque|GetBoardPreview) Casilla))
    (:then
      (bind _asally (Utilities|Casting|CastToAlly (Class|BoardPlayerController|GetSelectedAlly))
        (:then
          (bind _returnvalue_2 (Class|CharacterBase|GetTeam _ascharacter_base)))
        (:CastFailed
          _)))
    (:CastFailed
      _))
  (return (and (and (and (or (and (Utilities|Enum|Equal(Enum) _returnvalue "Enemy") (not (== _returnvalue_2 0))) (and (Utilities|Enum|Equal(Enum) _returnvalue "Ally") (== _returnvalue_2 0))) (Class|EgnisCombatLibrary|IsCardTargetinRange _cartapreview _asally _ascharacter_base Punto)) (or (not (Class|EgnisAbilityLibrary|HasRule _asally "(TagName=\"Rule.Targeting.Seeding\")")) (Utilities|Array|ContainsItem (Variables|PreviewAtaque|GetCasillasRangoAtaque) Casilla))) (stale _bsuccess))))

(fn ActualizarFuegoFatuo
  (if (and (Variables|Default|GetbFuegoFatuoActivo) (Utilities|IsValid (Variables|Default|GetPendingCard)))
    (bind _returnvalue (Class|WidgetLayoutLibrary|GetMousePositiononPlatform))
    (bind (_outhit _returnvalue_2) (Collision|LineTraceByChannel (.WorldLocation (Class|PlayerController|DeprojectScreenPositiontoWorld (.X (Math|Vector2D|BreakVector2D (.PixelPosition (Class|SlateBlueprintLibrary|AbsolutetoViewport _returnvalue)))) (.Y (Math|Vector2D|BreakVector2D (.PixelPosition (Class|SlateBlueprintLibrary|AbsolutetoViewport _returnvalue)))))) (+ (.WorldLocation (Class|PlayerController|DeprojectScreenPositiontoWorld (.X (Math|Vector2D|BreakVector2D (.PixelPosition (Class|SlateBlueprintLibrary|AbsolutetoViewport _returnvalue)))) (.Y (Math|Vector2D|BreakVector2D (.PixelPosition (Class|SlateBlueprintLibrary|AbsolutetoViewport _returnvalue)))))) (* (.WorldDirection (Class|PlayerController|DeprojectScreenPositiontoWorld (.X (Math|Vector2D|BreakVector2D (.PixelPosition (Class|SlateBlueprintLibrary|AbsolutetoViewport _returnvalue)))) (.Y (Math|Vector2D|BreakVector2D (.PixelPosition (Class|SlateBlueprintLibrary|AbsolutetoViewport _returnvalue)))))) 2e+05)) "TraceTypeQuery4" true 0 "None"))
    (if _returnvalue_2
      (if (Utilities|IsValid (Variables|FuegoFatuo|GetFuegoFatuo))
        (Transformation|SetWorldLocation (Variables|FuegoFatuo|GetFuegoFatuo) (+ (.ImpactPoint (Collision|BreakHitResult _outhit)) (* (.WorldDirection (Class|PlayerController|DeprojectScreenPositiontoWorld (.X (Math|Vector2D|BreakVector2D (.PixelPosition (Class|SlateBlueprintLibrary|AbsolutetoViewport _returnvalue)))) (.Y (Math|Vector2D|BreakVector2D (.PixelPosition (Class|SlateBlueprintLibrary|AbsolutetoViewport _returnvalue)))))) -4e+01)) false false)
        (else
          (bind _returnvalue_3 (Niagara|SpawnSystematLocation "/Game/GameDesign/Bruno/Card/FuegoFatuo/NS_FuegoFatuo.NS_FuegoFatuo" (+ (.ImpactPoint (Collision|BreakHitResult _outhit)) (* (.WorldDirection (Class|PlayerController|DeprojectScreenPositiontoWorld (.X (Math|Vector2D|BreakVector2D (.PixelPosition (Class|SlateBlueprintLibrary|AbsolutetoViewport _returnvalue)))) (.Y (Math|Vector2D|BreakVector2D (.PixelPosition (Class|SlateBlueprintLibrary|AbsolutetoViewport _returnvalue)))))) -4e+01))))
          (Variables|FuegoFatuo|SetFuegoFatuo _returnvalue_3))))
    (else
      (Variables|Default|SetbFuegoFatuoActivo false)
      (if (Utilities|IsValid (Variables|FuegoFatuo|GetFuegoFatuo))
        (Components|DestroyComponent (Variables|FuegoFatuo|GetFuegoFatuo))
        (Variables|FuegoFatuo|SetFuegoFatuo 0)))))

(fn ClickMoverIntentarMover
  (bind (_hitresult _returnvalue) (Game|Player|GetHitResultUnderCursorbyChannel "TraceTypeQuery4" true))
  ;[0.55 0.42 0.08] 1 - HAY ALGUNA PIEZA EN MODO CLICK?
  (if (Utilities|IsValid (Variables|MovimientoClick|GetPiezaModoClick))
    ;[0.1 0.3 0.55] 2 - CASILLA DEL TABLERO BAJO EL CURSOR
    (if (and _returnvalue (.ReturnValue (Class|Board|WorldPointtoTile (Variables|/Script/EgnisDef.CharacterBase|GetBoard (Variables|MovimientoClick|GetPiezaModoClick)) (.ImpactPoint (Collision|BreakHitResult _hitresult)))))
      ;[0.1 0.3 0.55] 3 - PEDIR EL MOVIMIENTO (guarda antes la posicion para el salto)
      (Variables|Default|SetPosInicial (Transformation|GetActorLocation (Variables|MovimientoClick|GetPiezaModoClick)))
      (bind _returnvalue_2 (Class|BoardPlayerController|RequestUnitMove (Variables|MovimientoClick|GetPiezaModoClick) (.OutTile (Class|Board|WorldPointtoTile (Variables|/Script/EgnisDef.CharacterBase|GetBoard (Variables|MovimientoClick|GetPiezaModoClick)) (.ImpactPoint (Collision|BreakHitResult _hitresult))))))
      (if _returnvalue_2
        ;[0.1 0.45 0.2] 4A - MOVIMIENTO VALIDO: salto, ocultar alcance y salir del modo click
        (Default|SaltarA (Variables|MovimientoClick|GetPiezaModoClick) (Variables|Default|GetPosInicial) (Class|CharacterBase|GetStandLocationforTile (Variables|MovimientoClick|GetPiezaModoClick) (.OutTile (Class|Board|WorldPointtoTile (Variables|/Script/EgnisDef.CharacterBase|GetBoard (Variables|MovimientoClick|GetPiezaModoClick)) (.ImpactPoint (Collision|BreakHitResult _hitresult))))))
        (bind _asbp_board (Utilities|Casting|CastToBP_Board (Variables|/Script/EgnisDef.CharacterBase|GetBoard (Variables|MovimientoClick|GetPiezaModoClick)) :!label _label))
        (Default|OcultarAlcance _asbp_board)
        (Variables|MovimientoClick|SetPiezaModoClick 0)
        (else
          ;[0.55 0.15 0.1] 4B - MOVIMIENTO RECHAZADO: si la pieza ya no puede mover se sale del modo click; si solo era una casilla invalida se mantiene
          (if (not (Class|BoardPlayerController|CanUnitMoveThisTurn (Variables|MovimientoClick|GetPiezaModoClick)))
            (goto _label)))))))

(fn ClickMoverAlSoltar
  (bind (_hitresult _returnvalue) (Game|Player|GetHitResultUnderCursorbyChannel "TraceTypeQuery4" true))
  (bind _piezaarrastrada (Variables|Default|GetPiezaArrastrada))
  (bind _impactpoint (Collision|BreakHitResult _hitresult))
  (bind _board (Variables|/Script/EgnisDef.CharacterBase|GetBoard _piezaarrastrada))
  (bind (_outtile _returnvalue_2) (Class|Board|WorldPointtoTile _board _impactpoint))
  ;[0.1 0.3 0.55] 1 - CLICK SIN ARRASTRAR?  La pieza se ha soltado sobre su propia casilla
  (if (and (and _returnvalue _returnvalue_2) (== (Class|Board|GetTileOccupant _board _outtile) (Variables|Default|GetPiezaArrastrada)))
    ;[0.55 0.42 0.08] 2 - YA ESTABA EN MODO CLICK ESTA PIEZA?
    (if (== (Variables|MovimientoClick|GetPiezaModoClick) (Variables|Default|GetPiezaArrastrada))
      ;[0.55 0.15 0.1] 3A - CANCELAR: segundo click en la misma pieza (o se ha arrastrado a otra casilla)
      (Variables|MovimientoClick|SetPiezaModoClick 0 :!label _label)
      (else
        ;[0.1 0.45 0.2] 3B - ACTIVAR MODO CLICK: guarda la pieza y deja su alcance a la vista
        (bind _output_get (Variables|MovimientoClick|SetPiezaModoClick (Variables|Default|GetPiezaArrastrada)))
        (bind _casillas (Default|ObtenerAlcance _output_get))
        (bind _asbp_board (Utilities|Casting|CastToBP_Board (Variables|/Script/EgnisDef.CharacterBase|GetBoard _output_get)))
        (Default|MostrarAlcance _asbp_board _casillas)))
    (else
      (goto _label))))

(fn ActualizarEnemigoBajoCursor
  ;[0.25 0.45 0.9] 1. Que enemigo hay bajo el raton (None si ninguno). Funciona en preparacion y en combate
  (bind _asbp_enemy_base (Utilities|Casting|CastToBP_Enemy_Base (.HitActor (Collision|BreakHitResult (.HitResult (Game|Player|GetHitResultUnderCursorbyChannel "TraceTypeQuery1" true)))))
    (:then
      _)
    (:CastFailed
      _))
  ;[0.9 0.15 0.1] 2. Si ha cambiado: apagar el anterior, guardar el nuevo y encenderlo (contorno intenso + barra de vida)
  (if (!= (Variables|Enemigos|Hover|GetEnemigoResaltado) _asbp_enemy_base)
    (if (Utilities|IsValid (Variables|Enemigos|Hover|GetEnemigoResaltado))
      (Default|ActualizarResaltado (Variables|Enemigos|Hover|GetEnemigoResaltado) false))
    (bind _output_get (Variables|Enemigos|Hover|SetEnemigoResaltado _asbp_enemy_base))
    (if (Utilities|IsValid _output_get)
      (Default|ActualizarResaltado _output_get true))))