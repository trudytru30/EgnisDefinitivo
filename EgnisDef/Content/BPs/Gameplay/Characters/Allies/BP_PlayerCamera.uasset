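; Player camera that plays an opening timeline transition, moving its pivot from an origin reference to an isometric view.
; Tick drives gated updates: W/S switch between an interpolated fixed top-down view and the saved start view, and mouse wheel sets two spring-arm zoom lengths.
; MOVE and test key T trigger camera shake and a click sound.
; A/D pivot rotation and damage shake (Sway) exist but are never called here.
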(event `Sway`
  (`PlayerController.ClientStartCameraShake` :`self` (`GameplayStatics.GetPlayerController` 0) :`Shake` "/Game/BPs/Camera/CameraDamageShake.CameraDamageShake_C"))

(event `self.ReceiveBeginPlay`
  (bind _camera (`self.Camera`))
  ; TopDownView
  (`self.Transition`)
  (set `self.InitialRotationCamera` (`SceneComponent.K2_GetComponentRotation` _camera))
  (set `self.IntialPositionCamera` (`SceneComponent.K2_GetComponentLocation` _camera)))

(event `TopDownView`
  (bind _camera (`self.Camera`))
  (bind _camera_2 (`self.Camera`))
  ; TopDownView
  (`/Engine/EditorBlueprintResources/StandardMacros.Gate` true :!label _label
    (:`Exit`
      (if (`self.W`)
        (`SceneComponent.K2_SetWorldLocationAndRotation` _camera (`KismetMathLibrary.VInterpTo` (`SceneComponent.GetSocketLocation` _camera_2 "None") (-850.0 -820.0 830.0) 5.0 5.0) (`KismetMathLibrary.RInterpTo` (`SceneComponent.GetSocketRotation` _camera_2 "None") (struct :`Pitch` -90.0) 5.0 5.0) true false)
        (elif (`self.S`)
          (`SceneComponent.K2_SetWorldLocationAndRotation` _camera (`self.IntialPositionCamera`) (`self.InitialRotationCamera`) false false))))))

(event `Key|W`
  (params (Key :type "Key Structure"))
  ; TopDownView
  (:`Pressed`
    (set `self.W` true)
    (set `self.S` false)
    (goto _label :!via `Open`))
  (:`Released`
    (set `self.W` false)
    (set `self.S` true)
    (goto _label :!via `Close`)))

(event `Key|S`
  (params (Key :type "Key Structure"))
  ; TopDownView
  (:`Pressed`
    (set `self.S` true)
    (set `self.W` false)
    (goto _label :!via `Open`))
  (:`Released`
    (set `self.S` false)
    (set `self.W` true)
    (goto _label :!via `Close`)))

(event `Rotate`
  (bind _pivote (`self.Pivote`))
  ; Rotation Arm
  (`/Engine/EditorBlueprintResources/StandardMacros.Gate` true :!label _label_2
    (:`Exit`
      (if (`self.Right`)
        (`SceneComponent.K2_AddLocalRotation` _pivote (`KismetMathLibrary.MakeRotator` 0.0 0.0 0.4) false false)
        (elif (`self.Left`)
          (`SceneComponent.K2_AddLocalRotation` _pivote (`KismetMathLibrary.MakeRotator` 0.0 0.0 -0.4) false false))))))

(event `self.ReceiveTick`
  (params (DeltaSeconds :type "Float (single-precision)"))
  (`self.Zooom`)
  (`self.TopDownView`))

(event `Key|D`
  (params (Key :type "Key Structure"))
  ; Rotation Arm
  (:`Pressed`
    (set `self.Right` true)
    (goto _label_2 :!via `Toggle`))
  (:`Released`
    (set `self.Right` false)
    (goto _label_2 :!via `Close`)))

(event `Key|A`
  (params (Key :type "Key Structure"))
  ; Rotation Arm
  (:`Pressed`
    (set `self.Left` true)
    (goto _label_2 :!via `Toggle`))
  (:`Released`
    (set `self.Left` false)
    (goto _label_2 :!via `Close`)))

(event `Zooom`
  ; Zoom
  (`/Engine/EditorBlueprintResources/StandardMacros.Gate` false :!label _label_3
    (:`Exit`
      (set `SpringArmComponent.TargetArmLength` (`KismetMathLibrary.FClamp` (`self.Zoom`) 10.0 300.0) (`self.SpringArm`)))))

(event `Key|T`
  (params (Key :type "Key Structure"))
  ; Move_feedback
  (:`Pressed`
    (`PlayerController.ClientStartCameraShake` :`self` (`GameplayStatics.GetPlayerController` 0) :`Scale` 2.0 :!label _label_4)
    (`GameplayStatics.PlaySoundAtLocation` "/Engine/VREditor/Sounds/UI/Click_on_Button.Click_on_Button" (-830.0 -790.0 10.0) (struct) 1.0 1.0 0.0 null null null null)))

(event `Key|MouseScrollUp`
  (params (Key :type "Key Structure"))
  ; Zoom
  (:`Pressed`
    (set `self.Zoom` 20.0)
    (goto _label_3 :!via `Close`))
  (:`Released`
    (goto _label_3 :!via `Toggle`)))

(event `MOVE`
  ; Move_feedback
  (goto _label_4))

(event `Key|MouseScrollDown`
  (params (Key :type "Key Structure"))
  ; Zoom
  (:`Pressed`
    (set `self.Zoom` 250.0)
    (goto _label_3 :!via `Close`))
  (:`Released`
    (goto _label_3 :!via `Open`)))

(event `Transition`
  (bind (_direction _output) (`Timeline|CameraTrans` :!via `PlayFromStart`)
    (:`Update`
      (`SceneComponent.K2_SetWorldTransform` (`self.Pivote`) (`KismetMathLibrary.TLerp` (`SceneComponent.K2_GetComponentToWorld` (`self.OriginRef`)) (`SceneComponent.K2_GetComponentToWorld` (`self.FinalRefIso`)) _output) true false))))

(fn `UserConstructionScript`)