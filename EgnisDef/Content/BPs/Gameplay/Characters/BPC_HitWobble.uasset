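; Actor component that wobbles its owner's mesh when an enemy applies a gameplay effect to it.
; It picks the tallest visible static mesh and rocks it about a local horizontal axis perpendicular to the attacker's direction.
; The angle follows an optional curve or a damped sine fallback.
; Tick runs only during a wobble, and repeat hits restart it from the saved base rotation, which is restored when it ends.
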(event `self.ReceiveBeginPlay`
  (bind _returnvalue (`self.GetOwner`))
  (`self.SetComponentTickEnabled` false)
  (bind (_asynctaskproxy _source) (`AbilityAsync_WaitGameplayEffectApplied.WaitGameplayEffectAppliedToActor` (`self.GetOwner`))
    (:`OnApplied`
      (if (`EgnisAbilityLibrary.AreEnemies` (`self.GetOwner`) _source)
        (if (`self.bWobbling`)
          (set `self.Axis` (`KismetMathLibrary.InverseTransformDirection` (`Actor.GetTransform` _returnvalue) (`KismetMathLibrary.Cross_VectorVector` (0.0 0.0 1.0) (`KismetMathLibrary.Conv_Vector2DToVector` (`KismetMathLibrary.Normal2D` (`KismetMathLibrary.Conv_VectorToVector2D` (- (`Actor.K2_GetActorLocation` _returnvalue) (`Actor.K2_GetActorLocation` _source))))))) :!label _label)
          (set `self.Elapsed` 0.0)
          (set `self.bWobbling` true)
          (`self.SetComponentTickEnabled` true)
          (else
            (`self.FindModel`)
            (if (`KismetSystemLibrary.IsValid` (`self.Target`))
              (set `self.BaseRotation` (`SceneComponent.RelativeRotation` (`self.Target`)))
              (goto _label))))))))

(event `self.ReceiveTick`
  (params (DeltaSeconds :type "Float (single-precision)"))
  (set `self.Elapsed` (+ (`self.Elapsed`) DeltaSeconds))
  (if (>= (`self.Elapsed`) (`self.Duration`))
    (`SceneComponent.K2_SetRelativeRotation` (`self.Target`) (`self.BaseRotation`) false false)
    (set `self.bWobbling` false)
    (`self.SetComponentTickEnabled` false)
    (else
      (if (`KismetSystemLibrary.IsValid` (`self.WobbleCurve`))
        (set `self.Angle` (* (`self.MaxAngle`) (`CurveFloat.GetFloatValue` (`self.WobbleCurve`) (`self.Elapsed`))))
        (else
          (set `self.Angle` (* (* (`self.MaxAngle`) (`KismetMathLibrary.Exp` (- 0.0 (* (`self.Damping`) (`self.Elapsed`))))) (`KismetMathLibrary.Sin` (* (* (`self.Frequency`) (`self.Elapsed`)) 6.283185))))))
      (`SceneComponent.K2_SetRelativeRotation` (`self.Target`) (`KismetMathLibrary.ComposeRotators` (`self.BaseRotation`) (`KismetMathLibrary.RotatorFromAxisAndAngle` (`self.Axis`) (`self.Angle`))) false false))))

(fn `FindModel`
  (set `self.BestHeight` -1.0)
  (for _array_element (`Actor.K2_GetComponentsByClass` (`self.GetOwner`) "/Script/Engine.StaticMeshComponent")
    (bind _z (.z (`.BoxExtent` (`KismetSystemLibrary.GetComponentBounds` _array_element))))
    (if (and (`SceneComponent.IsVisible` _array_element) (> _z (`self.BestHeight`)))
      (set `self.Target` _array_element)
      (set `self.BestHeight` _z))))