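; Grid board actor that draws the tiles and the highlight layers for destination, movement reach, attack range, area and deployment zone.
; The construction script fills an instanced tile mesh and fits a plane to the board bounds.
; Show/hide functions place colored or instanced markers at tile centers.
; On BeginPlay it computes deployable tiles from level data or tile type, flagging edges in per-instance custom data to outline only the zone's border.
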(event `self.ReceiveBeginPlay`
  ;[0.9 0.55 0.12] Despliegue: al empezar la partida (el tablero ya esta generado) se muestra el contorno de la zona
  (`self.MostrarZonaDespliegue`))

(fn `CalcularZonaDespliegue`
  ;[0.6 0.6 0.6] 1. Vaciar la zona anterior
  (`KismetArrayLibrary.Array_Clear` (`self.ZonaDespliegue`))
  ;[0.25 0.45 0.9] 2. Recorrer todas las casillas del tablero (filas Y, columnas X)
  (for _index (range (`self.BoardSizeY`))
    (for _index_2 (range (`self.BoardSizeX`))
      (bind _tilecoord (make `TileCoord` _index_2 _index))
      ;[0.9 0.55 0.12] 3. Si se puede desplegar en ella, guardarla en ZonaDespliegue
      (bind _esdedespliegue (`self.EsCasillaDeDespliegue` _tilecoord))
      (if _esdedespliegue
        (`KismetArrayLibrary.Array_Add` (`self.ZonaDespliegue`) _tilecoord)))))

(fn `EsCasillaDeDespliegue`
  (params (Casilla :type "TileCoord Structure"))
  (returns (EsDeDespliegue :type Boolean))
  (bind _currentleveldata (`self.CurrentLevelData`))
  ;[0.25 0.45 0.9] 1. Tiene Level Data el tablero?
  (if (`KismetSystemLibrary.IsValid` _currentleveldata)
    ;[0.9 0.55 0.12] 2a. Con nivel: regla del nivel (tipo de casilla + lejos de enemigos)
    (return (`LevelDataAsset.CanDeployOnTile` _currentleveldata Casilla))
    (else
      ;[0.6 0.6 0.6] 2b. Sin nivel: cualquier casilla pisable
      (return (`LevelDataAsset.IsDeployableTileType` (`self.GetTileType` Casilla))))))

(fn `MostrarAlcance`
  (params (Casillas :type "Array of TileCoord Structure"))
  (bind _returnvalue (* (`self.TileVisualSize`) 0.009))
  (`InstancedStaticMeshComponent.ClearInstances` (`self.MarcadoresAlcance`))
  (for _array_element Casillas
    (`InstancedStaticMeshComponent.AddInstance` (`self.MarcadoresAlcance`) (`KismetMathLibrary.MakeTransform` (+ (`self.TileToWorldCenter` _array_element) (0.0 0.0 1.5)) (struct) (`KismetMathLibrary.MakeVector` _returnvalue _returnvalue 1.0)) true)))

(fn `MostrarArea`
  (params (Casillas :type "Array of TileCoord Structure"))
  (`self.PintarCasillas` (`self.MarcadoresArea`) Casillas 1.8))

(fn `MostrarMarcador`
  (params (Casillas :type "TileCoord Structure") (Valida :type Boolean))
  (bind _marcador_destino (`self.Marcador Destino`))
  (`SceneComponent.K2_SetWorldLocation` _marcador_destino (+ (`self.TileToWorldCenter` Casillas) (0.0 0.0 2.0)) false false)
  (if Valida
    (`PrimitiveComponent.SetMaterial` _marcador_destino 0 "/AnimationSharing/AnimSharingGreen.AnimSharingGreen") ; CasillaDisponible
    (else
      (`PrimitiveComponent.SetMaterial` _marcador_destino 0 "/AnimationSharing/AnimSharingRed.AnimSharingRed") ; CasillaBloqueada
    ))
  (`SceneComponent.SetHiddenInGame` _marcador_destino false false))

(fn `MostrarRangoAtaque`
  (params (Casillas :type "Array of TileCoord Structure"))
  (`self.PintarCasillas` (`self.MarcadoresAtaque`) Casillas 1.6))

(fn `MostrarZonaDespliegue`
  (bind _marcadoresdespliegue (`self.MarcadoresDespliegue`))
  (bind _returnvalue (* (`self.TileVisualSize`) 0.01))
  ;[0.6 0.6 0.6] 1. Calcular la zona y borrar el contorno anterior
  (`self.CalcularZonaDespliegue`)
  (`InstancedStaticMeshComponent.ClearInstances` (`self.MarcadoresDespliegue`))
  ;[0.25 0.45 0.9] 2. Por cada casilla de la zona: colocar un plano en su centro (tamano exacto de casilla para que los bordes encajen)
  (for _array_element (`self.ZonaDespliegue`)
    (bind _returnvalue_2 (`InstancedStaticMeshComponent.AddInstance` _marcadoresdespliegue (`KismetMathLibrary.MakeTransform` (+ (`self.TileToWorldCenter` _array_element) (`KismetMathLibrary.MakeVector` 0.0 0.0 (`self.AlturaZonaDespliegue`))) (struct) (`KismetMathLibrary.MakeVector` _returnvalue _returnvalue 1.0)) true))
    ;[0.9 0.55 0.12] 3. Marcar que lados llevan linea (Custom Data 0..3). Solo donde la vecina NO es de la zona -> asi se ve solo el limite exterior
    (`InstancedStaticMeshComponent.SetCustomDataValue` _marcadoresdespliegue _returnvalue_2 0 (`self.TieneBorde` _array_element -1) false)
    (`InstancedStaticMeshComponent.SetCustomDataValue` _marcadoresdespliegue _returnvalue_2 1 (`self.TieneBorde` _array_element 1) false)
    (`InstancedStaticMeshComponent.SetCustomDataValue` _marcadoresdespliegue _returnvalue_2 2 (`self.TieneBorde` _array_element 0 -1) false)
    (`InstancedStaticMeshComponent.SetCustomDataValue` _marcadoresdespliegue _returnvalue_2 3 (`self.TieneBorde` _array_element 0 1) true)))

(fn `OcultarAlcance`
  (`InstancedStaticMeshComponent.ClearInstances` (`self.MarcadoresAlcance`)))

(fn `OcultarMarcador`
  (`SceneComponent.SetHiddenInGame` (`self.Marcador Destino`) true false))

(fn `OcultarRangoAtaque`
  (`InstancedStaticMeshComponent.ClearInstances` (`self.MarcadoresAtaque`))
  (`InstancedStaticMeshComponent.ClearInstances` (`self.MarcadoresArea`)))

(fn `OcultarZonaDespliegue`
  ;[0.9 0.55 0.12] Ocultar zona de despliegue: borra todas las casillas del contorno
  (`InstancedStaticMeshComponent.ClearInstances` (`self.MarcadoresDespliegue`)))

(fn `PintarCasillas`
  (params (Marcadores :type "InstancedStaticMeshComponent Object Reference") (Casillas :type "Array of TileCoord Structure") (AlturaZ :type "Float (double-precision)"))
  (bind _returnvalue (* (`self.TileVisualSize`) 0.009))
  (`InstancedStaticMeshComponent.ClearInstances` Marcadores)
  (for _array_element Casillas
    (`InstancedStaticMeshComponent.AddInstance` Marcadores (`KismetMathLibrary.MakeTransform` (+ (`self.TileToWorldCenter` _array_element) (`KismetMathLibrary.MakeVector` 0.0 0.0 AlturaZ)) (struct) (`KismetMathLibrary.MakeVector` _returnvalue _returnvalue 1.0)) true)))

(fn `TieneBorde`
  (params (Casilla :type "TileCoord Structure") (DireccionX :type Integer) (DireccionY :type Integer))
  (returns (Borde :type "Float (double-precision)"))
  (bind (_x _y) (break `TileCoord` Casilla))
  (return (`KismetMathLibrary.Conv_BoolToDouble` (not (`KismetArrayLibrary.Array_Contains` (`self.ZonaDespliegue`) (make `TileCoord` (+ _x DireccionX) (+ _y DireccionY)))))))

(fn `UserConstructionScript`
  (bind (_outcenter _outsize) (`self.GetBoardBounds`))
  (bind _plane (`self.Plane`))
  (bind _returnvalue (* (`self.TileVisualSize`) 0.01))
  (`InstancedStaticMeshComponent.ClearInstances` (`self.Tiles`))
  (for _index (range (`self.BoardSizeX`))
    (for _index_2 (range (`self.BoardSizeY`))
      (`InstancedStaticMeshComponent.AddInstance` (`self.Tiles`) (`KismetMathLibrary.MakeTransform` (+ (`self.TileToWorldCenter` (make `TileCoord` _index _index_2)) (0.0 0.0 1.0)) (struct) (`KismetMathLibrary.MakeVector` _returnvalue _returnvalue 1.0)) true)))
  (`SceneComponent.K2_SetWorldLocation` _plane _outcenter false false)
  (`SceneComponent.SetWorldScale3D` _plane (`KismetMathLibrary.MakeVector` (* (`KismetMathLibrary.BreakVector2D` _outsize) 0.1) (* (`.Y` (`KismetMathLibrary.BreakVector2D` _outsize)) 0.1) 1.0)))