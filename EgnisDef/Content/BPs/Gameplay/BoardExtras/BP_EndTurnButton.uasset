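; End-turn button on the game board that the player interacts with to end their turn in battle.
; One eased timeline sinks and spins the pivot while fading the emblem glow, then requests end turn through BoardPlayerController.
; The same timeline reverses to raise the button when the player's turn starts, or immediately if the turn did not end.
; It starts invisible and locked, and a Busy flag blocks input until the rise finishes and collision returns.
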(event `self.ReceiveBeginPlay`
  (bind _pivot (`self.Pivot`))
  (`SceneComponent.K2_SetRelativeLocationAndRotation` _pivot (0.0 0.0 -24.0) (struct :`Yaw` 360.0) false false)
  (`SceneComponent.SetVisibility` _pivot false true)
  (`PrimitiveComponent.SetCollisionEnabled` (`self.ButtonMesh`) "NoCollision")
  (bind _returnvalue (`PrimitiveComponent.CreateDynamicMaterialInstance` (`self.Emblem`) 0 null "None"))
  (set `self.EmblemMID` _returnvalue)
  (set `self.bHiddenForEnemyTurn` true)
  (set `self.bBusy` true)
  (`KismetSystemLibrary.DelayUntilNextTick`)
  (bind _asgame_manager (cast `GameManager` (`GameplayStatics.GetGameMode`)))
  (bind _returnvalue_2 (`BattleSceneManager.GetBattleManager` (`GameManager.GetBattleSceneManager` _asgame_manager)))
  (set `self.BattleManager` _returnvalue_2)
  (add `BattleManager.OnPlayerTurnStarted` _returnvalue_2 (delegate `HandlePlayerTurnStarted`)))

(event `self.Interactable.OnInteracted`
  (bind _buttonmesh (`self.ButtonMesh`))
  (if (and (not (`self.bBusy`)) (`BattleManager.IsPlayerTurn` (`self.BattleManager`)))
    (set `self.bBusy` true)
    (bind (_direction _alpha) (`Timeline|PressAnim` :!via `PlayFromStart` :!label _label)
      (:`Update`
        (bind _returnvalue (`KismetMathLibrary.Ease` 0.0 1.0 _alpha "SinusoidalInOut"))
        (`SceneComponent.K2_SetRelativeLocationAndRotation` (`self.Pivot`) (`KismetMathLibrary.MakeVector` 0.0 0.0 (* _returnvalue (`self.SinkDepth`))) (`KismetMathLibrary.MakeRotator` 0.0 0.0 (* _returnvalue (`self.SpinDegrees`))) false false)
        (`MaterialInstanceDynamic.SetScalarParameterValue` (`self.EmblemMID`) "GlowIntensity" (- 1.0 _returnvalue)))
      (:`Finished`
        (if (== _direction 0)
          (`SceneComponent.SetVisibility` (`self.Pivot`) true true)
          (`PrimitiveComponent.SetCollisionEnabled` _buttonmesh "NoCollision")
          (set `self.bHiddenForEnemyTurn` true)
          (bind _asboard_player_controller (cast `BoardPlayerController` (`GameplayStatics.GetPlayerController` 0))
            (:`then`
              (`BoardPlayerController.RequestEndTurn` _asboard_player_controller)
              (if (`BattleManager.IsPlayerTurn` (`self.BattleManager`))
                (set `self.bHiddenForEnemyTurn` false :!label _label_2)
                (`SceneComponent.SetVisibility` (`self.Pivot`) true true)
                (goto _label :!via `ReverseFromEnd`)))
            (:`CastFailed`
              (goto _label_2)))
          (else
            (`PrimitiveComponent.SetCollisionEnabled` _buttonmesh "QueryAndPhysics")
            (set `self.bBusy` false)))))))

(event `HandlePlayerTurnStarted`
  (if (`self.bHiddenForEnemyTurn`)
    (goto _label_2)))

(fn `UserConstructionScript`)