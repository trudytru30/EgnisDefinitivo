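; BP_BattleSceneManager shows and hides the battle scene's unit deployment UI and game HUD.
; Separate show events create the WBP_DeployUnits and WBP_GameHUD widgets, store references and add them to the viewport.
; Matching hide events remove the stored widgets from their parent, and each show call creates a fresh widget instance.
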(event `self.ShowDeploymentUI`
  (bind _returnvalue (`|CreateWidget` "/Game/GameDesign/Bruno/UI/seleccionPersonajes/WBP_DeployUnits.WBP_DeployUnits_C"))
  (bind _output_get (set `self.Deploy UI` _returnvalue))
  (`UserWidget.AddToViewport` _output_get 0))

(event `self.HideDeploymentUI`
  (`Widget.RemoveFromParent` (`self.Deploy UI`)))

(event `self.ShowHUD`
  (bind _returnvalue (`|CreateWidget` "/Game/UI/WBP_GameHUD.WBP_GameHUD_C"))
  (bind _output_get (set `self.HUD` _returnvalue))
  (`UserWidget.AddToViewport` _output_get 0))

(event `self.HideHUD`
  (`Widget.RemoveFromParent` (`self.HUD`)))