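; BP_Ally is an allied unit on a tile grid that moves by jumping and can show a green selection-style outline overlay.
; It stores its real movement pattern and range, keeps the move component locked at zero range, and restores them briefly for reach queries.
; SaltarA drives a timeline parabolic arc to the target at constant height, then writes landing position and time to a material parameter collection for a wave effect.
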(event `self.ReceiveBeginPlay`
  (bind _movecomp (`self.MoveComp`))
  (bind _movecomp_2 (`self.MoveComp`))
  ; Seteo Base
  (set `self.PatronReal` (`GridMovementComponent.movePattern` _movecomp_2))
  (set `self.RangoReal` (`GridMovementComponent.moveRange` _movecomp_2))
  (set `GridMovementComponent.movePattern` "Straight_WBlock" _movecomp)
  (set `GridMovementComponent.moveRange` 0 _movecomp))

(event `SaltarA`
  (params (Inicio :type "Vector Structure") (Destino :type "Vector Structure"))
  (bind _saltofin (`self.SaltoFin`))
  ; Movimiento Parabola
  (set `self.SaltoInicio` Inicio)
  (set `self.SaltoFin` (`KismetMathLibrary.MakeVector` (.x Destino) (.y Destino) (.z Inicio)))
  (bind (_direction _alpha) (`Timeline|Timeline` :!via `PlayFromStart`)
    (:`Update`
      (`self.K2_SetActorLocation` (+ (`KismetMathLibrary.VLerp` (`self.SaltoInicio`) _saltofin _alpha) (`KismetMathLibrary.MakeVector` 0.0 0.0 (* (* _alpha (- 1.0 _alpha)) (* (`self.AlturaSalto`) 4.0))))))
    (:`Finished`
      (`self.K2_SetActorLocation` _saltofin)
      ;; Onda pos caida
      (`KismetMaterialLibrary.SetVectorParameterValue` "/Game/Materials/MPC_Onda.MPC_Onda" "OndaCentro" (`KismetMathLibrary.Conv_VectorToLinearColor` _saltofin))
      (`KismetMaterialLibrary.SetScalarParameterValue` "/Game/Materials/MPC_Onda.MPC_Onda" "OndaInicio" (`KismetSystemLibrary.GetGameTimeInSeconds`)))))

(fn `ObtenerAlcance`
  (returns (Casillas :type "Array of TileCoord Structure"))
  (bind _movecomp (`self.MoveComp`))
  (set `GridMovementComponent.movePattern` (`self.PatronReal`) _movecomp)
  (set `GridMovementComponent.moveRange` (`self.RangoReal`) _movecomp)
  (bind _outtiles (`GridMovementComponent.getRachableTiles` _movecomp))
  (set `GridMovementComponent.movePattern` "Straight_WBlock" _movecomp)
  (set `GridMovementComponent.moveRange` 0 _movecomp)
  (return _outtiles))

(fn `PuedeIrA`
  (params (Casilla :type "TileCoord Structure"))
  (returns (Resultado :type Boolean))
  (bind _movecomp (`self.MoveComp`))
  (set `GridMovementComponent.movePattern` (`self.PatronReal`) _movecomp)
  (set `GridMovementComponent.moveRange` (`self.RangoReal`) _movecomp)
  (bind _returnvalue (`GridMovementComponent.canMoveToTile` _movecomp Casilla))
  (set `GridMovementComponent.movePattern` "Straight_WBlock" _movecomp)
  (set `GridMovementComponent.moveRange` 0 _movecomp)
  (return _returnvalue))

(fn `SetOutline`
  (params (Activo :type Boolean))
  (bind _staticmesh (`self.StaticMesh`))
  (if Activo
    (`MeshComponent.SetOverlayMaterial` _staticmesh "/Game/Migrate_Luis/Materials/Outline/MI_OutlineGreen.MI_OutlineGreen")
    (else
      (`MeshComponent.SetOverlayMaterial` _staticmesh null))))

(fn `UserConstructionScript`)