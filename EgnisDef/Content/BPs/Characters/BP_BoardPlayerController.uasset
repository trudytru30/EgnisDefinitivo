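; Player controller for a tile-board game that handles selecting and moving ally pieces, refreshing the hand HUD and ending turns.
; Left click picks and outlines an ally.
; Right-click drag lifts an unmoved ally, shows its range and a validity marker via cursor traces, then jumps it to a valid tile or snaps it back.
; Each ally moves once per turn; TerminarTurno resets those flags and requests turn end.
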(event `self.BP_RefreshHandUI`
  (bind _aswbp_game_hud (cast `/Game/UI/WBP_GameHUD` (`self.HUD WIdget`)))
  (`/Game/UI/WBP_GameHUD.SetHand` _aswbp_game_hud (`self.GetCurrentHand`)))

(event `EnhancedInput|/Game/Inputs/IA_LeftClick`
  (params (ActionValue :type Boolean) (ElapsedSeconds :type "Float (double-precision)") (TriggeredSeconds :type "Float (double-precision)") (InputAction :type "InputAction Object Reference" :default "/Game/Inputs/IA_LeftClick.IA_LeftClick"))
  (bind _piezaseleccionada (`self.PiezaSeleccionada`))
  ; Outline Pieza
  (:`Started`
    (bind _asbp_ally (cast `/Game/BPs/Characters/BP_Ally` (`.HitActor` (`GameplayStatics.BreakHitResult` (`self.GetHitResultUnderCursorByChannel` "TraceTypeQuery3")))))
    (if (`KismetSystemLibrary.IsValid` _piezaseleccionada)
      (`/Game/BPs/Characters/BP_Ally.SetOutline` _piezaseleccionada true))
    (bind _output_get (set `self.PiezaSeleccionada` _asbp_ally))
    (`/Game/BPs/Characters/BP_Ally.SetOutline` _output_get true)))

(event `EnhancedInput|/Game/Inputs/IA_RightClick`
  (params (ActionValue :type Boolean) (ElapsedSeconds :type "Float (double-precision)") (TriggeredSeconds :type "Float (double-precision)") (InputAction :type "InputAction Object Reference" :default "/Game/Inputs/IA_RightClick.IA_RightClick"))
  (bind (_hitresult _returnvalue) (`self.GetHitResultUnderCursorByChannel` "TraceTypeQuery4"))
  (bind (_hitresult_2 _returnvalue_2) (`self.GetHitResultUnderCursorByChannel` "TraceTypeQuery4"))
  (bind _piezaarrastrada (`self.PiezaArrastrada`))
  (bind _piezaarrastrada_2 (`self.PiezaArrastrada`))
  (bind _posinicial (`self.PosInicial`))
  (bind _board (`CharacterBase.Board` _piezaarrastrada_2))
  (bind (_outtile _returnvalue_3) (`Board.WorldPointToTile` _board (`.ImpactPoint` (`GameplayStatics.BreakHitResult` _hitresult))))
  (bind (_outtile_2 _returnvalue_4) (`Board.WorldPointToTile` _board (`.ImpactPoint` (`GameplayStatics.BreakHitResult` _hitresult_2))))
  (bind _asbp_board (cast `/Game/BPs/Board/BP_Board` _board :!pure true))
  ; Preview Mov
  (:`Triggered`
    (if (`KismetSystemLibrary.IsValid` _piezaarrastrada_2)
      (if (and _returnvalue _returnvalue_3)
        (bind _resultado (`/Game/BPs/Characters/BP_Ally.PuedeIrA` (`self.PiezaArrastrada`) _outtile))
        (`/Game/BPs/Board/BP_Board.MostrarMarcador` _asbp_board _outtile _resultado)
        (else
          (`/Game/BPs/Board/BP_Board.OcultarMarcador` _asbp_board)))))
  (:`Started`
    (bind _asbp_ally (cast `/Game/BPs/Characters/BP_Ally` (`.HitActor` (`GameplayStatics.BreakHitResult` (`self.GetHitResultUnderCursorByChannel` "TraceTypeQuery3")))))
    (if (not (`/Game/BPs/Characters/BP_Ally.bMovidoEsteTurno` _asbp_ally))
      (bind _output_get (set `self.PiezaArrastrada` _asbp_ally))
      (bind _output_get_2 (set `self.PosInicial` (`self.K2_GetActorLocation` _output_get)))
      (`self.K2_SetActorLocation` _output_get (+ _output_get_2 (0.0 0.0 25.0)) false false)
      (bind _casillas (`/Game/BPs/Characters/BP_Ally.ObtenerAlcance` _output_get))
      (`/Game/BPs/Board/BP_Board.MostrarAlcance` _asbp_board _casillas)))
  (:`Completed`
    (if (`KismetSystemLibrary.IsValid` _piezaarrastrada_2)
      (`/Game/BPs/Board/BP_Board.OcultarMarcador` _asbp_board)
      (`/Game/BPs/Board/BP_Board.OcultarAlcance` _asbp_board)
      (if (and _returnvalue_2 _returnvalue_4)
        (bind _resultado_2 (`/Game/BPs/Characters/BP_Ally.PuedeIrA` _piezaarrastrada _outtile_2))
        (if _resultado_2
          (bind _returnvalue_5 (`CharacterBase.SetCurrentTile` _piezaarrastrada _outtile_2))
          (if _returnvalue_5
            (`/Game/BPs/Characters/BP_Ally.SaltarA` _piezaarrastrada _posinicial (`Board.TileToWorldCenter` (`CharacterBase.Board` _piezaarrastrada) _outtile_2))
            (set `/Game/BPs/Characters/BP_Ally.bMovidoEsteTurno` true _piezaarrastrada)
            (set `self.Ya Movio Este Turno` true)
            (else
              (`self.K2_SetActorLocation` _piezaarrastrada _posinicial false false :!label _label)))
          (else
            (goto _label)))
        (else
          (goto _label)))
      (set `self.PiezaArrastrada` null))))

(fn `ReiniciarMovimientos`
  (bind _outactors (`GameplayStatics.GetAllActorsOfClass` "/Game/BPs/Characters/BP_Ally.BP_Ally_C"))
  (for _array_element _outactors
    (set `/Game/BPs/Characters/BP_Ally.bMovidoEsteTurno` false _array_element)))

(fn `TerminarTurno`
  (set `self.Ya Movio Este Turno` false)
  (`self.ReiniciarMovimientos`)
  (`self.RequestEndTurn`))

(fn `UserConstructionScript`)