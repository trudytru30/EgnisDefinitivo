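; BP_BattleSceneManager controls which UI screens appear during a board battle, creating and removing deployment, HUD and end-of-battle widgets.
; Deployment and HUD widgets are stored for later removal, and hiding deployment also tells BP_Board to hide its deployment zone outline.
; ShowHUD also hands the HUD to BP_BoardPlayerController, while ShowRewardsUI only shows a death screen on a loss and does nothing on a win.
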(event `self.ShowDeploymentUI`
  (bind _returnvalue (`|CreateWidget` "/Game/GameDesign/Bruno/UI/seleccionPersonajes/WBP_DeployUnits.WBP_DeployUnits_C"))
  (bind _output_get (set `self.Deploy UI` _returnvalue))
  (`UserWidget.AddToViewport` _output_get 0))

(event `self.HideDeploymentUI`
  (`Widget.RemoveFromParent` (`self.Deploy UI`))
  ;[0.9 0.55 0.12] Fin del despliegue: ocultar el contorno de la zona de despliegue del tablero
  (bind _returnvalue (`GameplayStatics.GetActorOfClass` self "/Game/BPs/Gameplay/Environment/Board/BP_Board.BP_Board_C"))
  (`/Game/BPs/Gameplay/Environment/Board/BP_Board.OcultarZonaDespliegue` _returnvalue))

(event `self.ShowHUD`
  (bind _returnvalue (`|CreateWidget` "/Game/BPs/Gameplay/UI/WBP_GameHUD.WBP_GameHUD_C"))
  (bind _output_get (set `self.HUD` _returnvalue))
  (bind _asbp_board_player_controller (cast `/Game/BPs/Gameplay/Characters/Allies/BP_BoardPlayerController` (`GameplayStatics.GetPlayerController` 0)))
  (bind _output_get_2 (set `/Game/BPs/Gameplay/Characters/Allies/BP_BoardPlayerController.HUD WIdget` _output_get _asbp_board_player_controller))
  (`UserWidget.AddToViewport` _output_get_2 0))

(event `self.HideHUD`
  (`Widget.RemoveFromParent` (`self.HUD`)))

(event `self.ShowRewardsUI`
  (params (bPlayerWon :type Boolean))
  (if (not bPlayerWon)
    (bind _returnvalue (`|CreateWidget` "/Game/GameDesign/Bruno/UI/Menus/WBP_DeathUI.WBP_DeathUI_C"))
    (`UserWidget.AddToViewport` _returnvalue 0)))